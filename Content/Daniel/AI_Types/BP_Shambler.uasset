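; Shambler enemy AI that wanders, closes on the player once perceived, and performs a placeholder melee attack.
; A 0.1-second timer re-runs the state logic, which only acts when an on-screen check passes.
; AI perception sets FoundPlayer, while construction-built min and max spheres set and clear IsInRange with hysteresis, together choosing Moving or Attacking.
; Attacking stops movement, turns toward the player, prints a message and waits briefly.
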(event `self.ReceiveBeginPlay`
  (`self.AIRun`))

(event `self.AIRun`
  (`KismetSystemLibrary.K2_SetTimerDelegate` (delegate `self.AIRun`) 0.1 true)
  (bind _newparam2 (`self.CheckToSeeOnScreen` (`GameplayStatics.GetPlayerController` 0) self))
  (if _newparam2
    (if (and (`self.FoundPlayer`) (`self.IsInRange`))
      (set `self.AI State` "NewEnumerator2")
      (else
        (set `self.AI State` "NewEnumerator1")))
    (switch `/Game/Daniel/AI_States` (`self.AI State`)
      (:`NewEnumerator0`
        (`KismetSystemLibrary.Delay` 3.0)
        (set `self.AI State` "NewEnumerator1"))
      (:`NewEnumerator1`
        (if (or (`self.IsMoving`) (`self.Is Attacking`))
          _
          (elif (`self.FoundPlayer`)
            (`self.Get In Range`)
            (else
              (`self.Movement` null self)))))
      (:`NewEnumerator2`
        (if (not (`self.Is Attacking`))
          (`self.Attack`))))))

(event `Attack`
  (bind _capsulecomponent (`self.CapsuleComponent`))
  (bind (_returnvalue_roll _returnvalue_pitch) (`KismetMathLibrary.BreakRotator` (`SceneComponent.K2_GetComponentRotation` _capsulecomponent)))
  (bind (_returnvalue_roll_2 _returnvalue_pitch_2 _returnvalue_yaw) (`KismetMathLibrary.BreakRotator` (`KismetMathLibrary.FindLookAtRotation` (`SceneComponent.K2_GetComponentLocation` (`self.SkeletalMesh`)) (`self.K2_GetActorLocation` (`GameplayStatics.GetPlayerCharacter` 0)))))
  (set `self.Is Attacking` true)
  (`self.AI Stop`)
  (`SceneComponent.K2_SetWorldRotation` _capsulecomponent (`KismetMathLibrary.MakeRotator` _returnvalue_roll _returnvalue_pitch _returnvalue_yaw) false false)
  (`KismetSystemLibrary.PrintString` "Melee attack")
  (`KismetSystemLibrary.Delay` 1.0)
  (set `self.Is Attacking` false))

(event `Get In Range`
  (`self.Movement` (`GameplayStatics.GetPlayerCharacter` 0) self))

(event `self.Min Range.OnComponentBeginOverlap`
  (params (OverlappedComponent :type "PrimitiveComponent Object Reference") (OtherActor :type "Actor Object Reference") (OtherComp :type "PrimitiveComponent Object Reference") (OtherBodyIndex :type Integer) (bFromSweep :type Boolean) (SweepResult :type "HitResult Structure (by ref)"))
  (if (== OtherActor (`GameplayStatics.GetPlayerCharacter` 0))
    (set `self.IsInRange` true)))

(event `self.Max Range.OnComponentEndOverlap`
  (params (OverlappedComponent :type "PrimitiveComponent Object Reference") (OtherActor :type "Actor Object Reference") (OtherComp :type "PrimitiveComponent Object Reference") (OtherBodyIndex :type Integer))
  (if (== OtherActor (`GameplayStatics.GetPlayerCharacter` 0))
    (set `self.IsInRange` false)))

(event `self.AIPerception.OnTargetPerceptionUpdated`
  (params (Actor :type "Actor Object Reference") (Stimulus :type "AIStimulus Structure"))
  (if (== Actor (`GameplayStatics.GetPlayerCharacter` 0))
    (if Stimulus_bSuccessfullySensed
      (set `self.FoundPlayer` true)
      (else
        (set `self.FoundPlayer` false)))))

(event `self.AIPerception.OnTargetPerceptionForgotten`
  (params (Actor :type "Actor Object Reference"))
  (if (== Actor (`GameplayStatics.GetPlayerCharacter` 0))
    (set `self.FoundPlayer` false)))

(fn `UserConstructionScript`
  (bind _returnvalue_location (`KismetMathLibrary.BreakTransform` (`SceneComponent.GetRelativeTransform` (`self.Mesh`))))
  (bind _returnvalue_location_2 (`KismetMathLibrary.BreakTransform` (`SceneComponent.GetRelativeTransform` (`self.Mesh`))))
  (`parent.UserConstructionScript`)
  (bind _returnvalue (`AddComponent|NODE_AddSphereComponent-0` :`RelativeTransform` (`KismetMathLibrary.MakeTransform` _returnvalue_location_2)))
  (bind _output_get (set `self.Max Range` _returnvalue))
  (`SphereComponent.SetSphereRadius` _output_get (`self.Attack Range Max`) true)
  (bind _returnvalue_2 (`AddComponent|NODE_AddSphereComponent-1` :`RelativeTransform` (`KismetMathLibrary.MakeTransform` _returnvalue_location)))
  (bind _output_get_2 (set `self.Min Range` _returnvalue_2))
  (`SphereComponent.SetSphereRadius` _output_get_2 (`self.Attack Range Min`) true))