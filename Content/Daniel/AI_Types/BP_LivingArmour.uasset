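; Living Armour enemy AI Blueprint that spawns a sword actor at its arrow component and attaches it on BeginPlay.
; While on screen, a timer-driven AIRun switches between moving and attacking using player detection and the MaxRange sphere, closing in, wandering or retrieving the sword.
; MinRange tracks melee range and can reattach the sword.
; Attacks are unfinished: melee and ranged events are empty, the melee call is disabled, and sword-swing timelines are unconnected.
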(event `self.ReceiveBeginPlay`
  (bind _arrow1 (`self.Arrow1`))
  (bind _returnvalue (`|SpawnActorFromClass` "/Game/Daniel/BP_LivingArmourSword.BP_LivingArmourSword_C" (`KismetMathLibrary.MakeTransform` (`SceneComponent.K2_GetComponentLocation` _arrow1) (`SceneComponent.K2_GetComponentRotation` _arrow1)) "Undefined" "MultiplyWithRoot" null 1.0 null null))
  (bind _output_get (set `self.Sword` _returnvalue))
  (`self.K2_AttachToActor` _output_get self "None" "KeepWorld" "KeepWorld" "KeepWorld" true)
  (`parent.ReceiveBeginPlay`))

(event `self.AIRun`
  (`KismetSystemLibrary.K2_SetTimerDelegate` (delegate `self.AIRun`) 0.1 true)
  (bind _newparam2 (`self.CheckToSeeOnScreen` (`GameplayStatics.GetPlayerController` 0) self))
  (if _newparam2
    (if (and (`self.FoundPlayer`) (`self.IsInRange`))
      (set `self.AI State` "NewEnumerator2")
      (else
        (set `self.AI State` "NewEnumerator1")))
    (switch `/Game/Daniel/AI_States` (`self.AI State`)
      (:`NewEnumerator0`
        (`KismetSystemLibrary.Delay` 3.0)
        (set `self.AI State` "NewEnumerator1"))
      (:`NewEnumerator1`
        (if (`self.IsMoving`)
          _
          (elif (`self.IsSwordEquipped`)
            (if (`self.FoundPlayer`)
              (`self.Get In Range`)
              (else
                (`self.Movement` null self)))
            (else
              (`self.GetSword`)))))
      (:`NewEnumerator2`
        (if (not true)
          (`self.Melee Attack`))))))

(event `self.Min Range.OnComponentBeginOverlap`
  (params (OverlappedComponent :type "PrimitiveComponent Object Reference") (OtherActor :type "Actor Object Reference") (OtherComp :type "PrimitiveComponent Object Reference") (OtherBodyIndex :type Integer) (bFromSweep :type Boolean) (SweepResult :type "HitResult Structure (by ref)"))
  (if (== OtherActor (`GameplayStatics.GetPlayerCharacter` 0))
    (set `self.IsMeleeRange` true)))

(event `self.Min Range.OnComponentEndOverlap`
  (params (OverlappedComponent :type "PrimitiveComponent Object Reference") (OtherActor :type "Actor Object Reference") (OtherComp :type "PrimitiveComponent Object Reference") (OtherBodyIndex :type Integer))
  (if (== OtherActor (`GameplayStatics.GetPlayerCharacter` 0))
    (set `self.IsMeleeRange` false)
    (elif (not (== (`self.GetAttachParentActor` (`self.Sword`)) self))
      (`self.K2_AttachToActor` (`self.Sword`) self "None" "KeepWorld" "KeepWorld" "KeepWorld" true))))

(event `Ranged Attack`)

(event `self.Max Range.OnComponentBeginOverlap`
  (params (OverlappedComponent :type "PrimitiveComponent Object Reference") (OtherActor :type "Actor Object Reference") (OtherComp :type "PrimitiveComponent Object Reference") (OtherBodyIndex :type Integer) (bFromSweep :type Boolean) (SweepResult :type "HitResult Structure (by ref)"))
  (if (== OtherActor (`GameplayStatics.GetPlayerCharacter` 0))
    (set `self.IsInRange` true)))

(event `self.Max Range.OnComponentEndOverlap`
  (params (OverlappedComponent :type "PrimitiveComponent Object Reference") (OtherActor :type "Actor Object Reference") (OtherComp :type "PrimitiveComponent Object Reference") (OtherBodyIndex :type Integer))
  (if (== OtherActor (`GameplayStatics.GetPlayerCharacter` 0))
    (set `self.IsInRange` false)))

(event `Melee Attack`)

(event `GetSword`
  (`self.AI Stop`)
  (`self.Movement` (`self.Sword`) self))

(fn `UserConstructionScript`
  (`parent.UserConstructionScript`)
  (`SphereComponent.SetSphereRadius` (`self.Min Range`) 150.0 true)
  (`SphereComponent.SetSphereRadius` (`self.Max Range`) 1000.0 true))