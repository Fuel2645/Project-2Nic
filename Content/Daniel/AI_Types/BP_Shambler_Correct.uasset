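; Shambler melee enemy that roams or closes on the player and attacks in range while a specific limb is active.
; A looping timer runs its Idle/Moving/Attacking state logic, gated by an on-screen check.
; Attacks track the player briefly, then chained timelines sweep the PointLight of an attached BP_ShamblerAttack actor forward, sideways and back.
; That attack actor spawns on BeginPlay and is destroyed with the Shambler on death.
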(event `self.ReceiveBeginPlay`
  (bind _arrow1 (`self.Arrow1`))
  (bind _returnvalue (`|SpawnActorFromClass` "/Game/Daniel/BP_ShamblerAttack.BP_ShamblerAttack_C" (`KismetMathLibrary.MakeTransform` (`SceneComponent.K2_GetComponentLocation` _arrow1) (`SceneComponent.K2_GetComponentRotation` _arrow1)) "AlwaysSpawn" "MultiplyWithRoot" null 0.5 self null))
  (bind _output_get (set `self.MeleeActor` _returnvalue))
  (`self.K2_AttachToActor` _output_get self "None" "KeepWorld" "KeepWorld" "KeepWorld" true)
  (`self.AIRun`))

(event `self.AIRun`
  (bind _bpc_hp (`self.BPC_HP`))
  (bind _bpc_hp_2 (`self.BPC_HP`))
  (`KismetSystemLibrary.K2_SetTimerDelegate` (delegate `self.AIRun`) 0.1 true)
  (bind _newparam2 (`self.CheckToSeeOnScreen` (`GameplayStatics.GetPlayerController` 0) self))
  (if _newparam2
    (if (and (`self.FoundPlayer`) (`self.IsInRange`))
      (if (`/Game/Design_Luke/BPC_HP.LimbActiveCheck` _bpc_hp (`|GetArrayItem` (`/Game/Design_Luke/BPC_HP.LimbNames` _bpc_hp) 2))
        (set `self.AI State` "NewEnumerator2")
        (else
          (set `self.AI State` "NewEnumerator1" :!label _label)))
      (else
        (goto _label)))
    (switch `/Game/Daniel/AI_States` (`self.AI State`)
      (:`NewEnumerator0`
        (`KismetSystemLibrary.Delay` 3.0)
        (set `self.AI State` "NewEnumerator1"))
      (:`NewEnumerator1`
        (if (not (or (`self.IsMoving`) (`self.Is Attacking`)))
          (if (`self.FoundPlayer`) :!label _label_2
            (`self.Get In Range`)
            (else
              (`self.Movement` null self)))))
      (:`NewEnumerator2`
        (if (`self.Is Attacking`)
          _
          (elif (`/Game/Design_Luke/BPC_HP.LimbActiveCheck` _bpc_hp_2 (`|GetArrayItem` (`/Game/Design_Luke/BPC_HP.LimbNames` _bpc_hp_2) 2))
            (`self.Attack`)
            (else
              (goto _label_2))))))))

(event `self.Attack`
  (bind _capsulecomponent (`self.CapsuleComponent`))
  (bind _capsulecomponent_2 (`self.CapsuleComponent`))
  (bind (_returnvalue_roll _returnvalue_pitch) (`KismetMathLibrary.BreakRotator` (`SceneComponent.K2_GetComponentRotation` _capsulecomponent)))
  (bind (_returnvalue_roll_2 _returnvalue_pitch_2) (`KismetMathLibrary.BreakRotator` (`SceneComponent.K2_GetComponentRotation` _capsulecomponent_2)))
  (bind _pointlight (`/Game/Design_Luke/ProjectileChildren/BP_ParentProjectile.PointLight` (`self.MeleeActor`)))
  (bind _pointlight_2 (`/Game/Design_Luke/ProjectileChildren/BP_ParentProjectile.PointLight` (`self.MeleeActor`)))
  (bind _pointlight_3 (`/Game/Design_Luke/ProjectileChildren/BP_ParentProjectile.PointLight` (`self.MeleeActor`)))
  (bind (_returnvalue_roll_3 _returnvalue_pitch_3 _returnvalue_yaw) (`KismetMathLibrary.BreakRotator` (`KismetMathLibrary.FindLookAtRotation` (`SceneComponent.K2_GetComponentLocation` (`self.Mesh`)) (`self.K2_GetActorLocation` (`GameplayStatics.GetPlayerPawn` 0)))))
  (bind (_returnvalue_roll_4 _returnvalue_pitch_4 _returnvalue_yaw_2) (`KismetMathLibrary.BreakRotator` (`KismetMathLibrary.FindLookAtRotation` (`SceneComponent.K2_GetComponentLocation` (`self.Mesh`)) (`self.K2_GetActorLocation` (`GameplayStatics.GetPlayerCharacter` 0)))))
  (set `self.Is Attacking` true)
  (`self.AI Stop`)
  (bind _returnvalue (`KismetSystemLibrary.K2_SetTimerDelegate` (delegate `self.Attack`) 0.1 true))
  (if (not (`self.IsMelleee`))
    (`SceneComponent.K2_SetWorldRotation` _capsulecomponent (`KismetMathLibrary.MakeRotator` _returnvalue_roll _returnvalue_pitch _returnvalue_yaw_2) false false)
    (bind _result (`/Engine/EditorBlueprintResources/StandardMacros.IncrementInt` (`self.LoopCount`))
      (:`  `
        (if (not (<= _result 6))
          (`KismetSystemLibrary.K2_PauseTimerHandle` _returnvalue)
          (if (`self.IsInRange`)
            (set `self.IsMelleee` true)
            (`SceneComponent.K2_SetWorldRotation` _capsulecomponent_2 (`KismetMathLibrary.MakeRotator` _returnvalue_roll_2 _returnvalue_pitch_2 _returnvalue_yaw) false false)
            (bind (_direction _newtrack_0) (`Timeline|Timeline` :!via `PlayFromStart`)
              (:`Update`
                (`SceneComponent.K2_SetWorldLocation` _pointlight_3 (`KismetMathLibrary.VLerp` (`SceneComponent.K2_GetComponentLocation` _pointlight_3) (+ (`SceneComponent.K2_GetComponentLocation` _pointlight_3) (* (`SceneComponent.GetForwardVector` _pointlight_3) 3.0)) _newtrack_0) false false))
              (:`Finished`
                (bind (_direction_2 _npcs) (`Timeline|SideAttack` :!via `PlayFromStart`)
                  (:`Update`
                    (`SceneComponent.K2_SetWorldLocation` _pointlight_2 (`KismetMathLibrary.VLerp` (`SceneComponent.K2_GetComponentLocation` _pointlight_2) (+ (`SceneComponent.K2_GetComponentLocation` _pointlight_2) (* (* (`SceneComponent.GetRightVector` _pointlight_2) -1.0) 5.0)) _npcs) false false))
                  (:`Finished`
                    (bind (_direction_3 _npcs_2) (`Timeline|Timeline_0` :!via `PlayFromStart`)
                      (:`Update`
                        (`SceneComponent.K2_SetWorldLocation` _pointlight (`KismetMathLibrary.VLerp` (`SceneComponent.K2_GetComponentLocation` _pointlight) (`SceneComponent.K2_GetComponentLocation` (`self.Arrow1`)) _npcs_2) false false))
                      (:`Finished`
                        (`KismetSystemLibrary.Delay` 1.0)
                        (set `self.Is Attacking` false)
                        (set `self.IsMelleee` false)
                        (set `self.LoopCount` 0)))))))
            (else
              (`KismetSystemLibrary.Delay` 1.0)
              (set `self.AI State` "NewEnumerator1")
              (set `self.Is Attacking` false)
              (set `self.IsMelleee` false)
              (set `self.LoopCount` 0))))))))

(event `/Game/Design_Luke/Combat_Interface.Die`
  (`self.K2_DestroyActor` (`self.MeleeActor`))
  (`self.K2_DestroyActor`))

(fn `UserConstructionScript`
  (set `self.Attack Range Min` 100.0)
  (set `self.Attack Range Max` 100.0)
  (`parent.UserConstructionScript`))