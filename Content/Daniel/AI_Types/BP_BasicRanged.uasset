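; BP_BasicRanged is a basic ranged AI type whose Attack event spawns an actor, presumably a projectile.
; Attack sets an Isattacking flag, waits briefly, then always spawns the actor at double scale, placed at the Arrow1 component and rotated to match the Mesh.
; After a second short delay it clears the flag; the file itself holds no targeting or movement logic.
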(event `self.Attack`
  (set `self.Isattacking` true)
  (`KismetSystemLibrary.Delay` 0.5)
  (`|SpawnActorFromClass` "/Game/Design_Luke/ProjectileChildren/RangedAttacks/BP_Bolt_Projectile_Child.BP_Bolt_Projectile_Child_C" (`KismetMathLibrary.MakeTransform` (`SceneComponent.K2_GetComponentLocation` (`self.Arrow1`)) (`SceneComponent.K2_GetComponentRotation` (`self.Mesh`)) (2.0 2.0 2.0)) "AlwaysSpawn" "MultiplyWithRoot" null 1.0 null null)
  (`KismetSystemLibrary.Delay` 0.5)
  (set `self.Isattacking` false))

(fn `UserConstructionScript`
  (`parent.UserConstructionScript`))