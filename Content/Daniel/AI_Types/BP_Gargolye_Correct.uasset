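; Gargoyle enemy AI that stays dormant until the player overlaps a detection sphere built in the construction script, then roams, closes range and attacks.
; A 0.1-second timer drives the Idle/Moving/Attacking state logic, gated by an on-screen check.
; Attacks repeatedly turn the capsule toward the player for several timer ticks, then run a Timeline forward dash with an attached cone projectile that is destroyed when the dash ends.
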(event `self.AIRun`
  (`KismetSystemLibrary.K2_SetTimerDelegate` (delegate `self.AIRun`) 0.1 true)
  (bind _newparam2 (`self.CheckToSeeOnScreen` (`GameplayStatics.GetPlayerController` 0) self))
  (if _newparam2
    (if (`self.IsAnimated`)
      (if (and (`self.FoundPlayer`) (`self.IsInRange`))
        (set `self.AI State` "NewEnumerator2")
        (else
          (set `self.AI State` "NewEnumerator1")))
      (switch `/Game/Daniel/AI_States` (`self.AI State`)
        (:`NewEnumerator0`
          (`KismetSystemLibrary.Delay` 3.0)
          (set `self.AI State` "NewEnumerator1"))
        (:`NewEnumerator1`
          (if (or (`self.IsMoving`) (`self.Is Attacking`))
            _
            (elif (`self.FoundPlayer`)
              (`self.Get In Range`)
              (else
                (`self.Movement` null self)))))
        (:`NewEnumerator2`
          (if (not (`self.Is Attacking`))
            (`self.Attack`)))))))

(event `self.Animation Detection .OnComponentBeginOverlap`
  (params (OverlappedComponent :type "PrimitiveComponent Object Reference") (OtherActor :type "Actor Object Reference") (OtherComp :type "PrimitiveComponent Object Reference") (OtherBodyIndex :type Integer) (bFromSweep :type Boolean) (SweepResult :type "HitResult Structure (by ref)"))
  (if (and (== OtherActor (`GameplayStatics.GetPlayerCharacter` 0)) (not (`self.IsAnimated`)))
    (`KismetSystemLibrary.PrintString` "Animated animation")
    (set `self.IsAnimated` true)))

(event `self.ReceiveBeginPlay`
  (`self.AIRun`))

(event `self.Attack`
  (bind _capsulecomponent (`self.CapsuleComponent`))
  (bind _arrow1 (`self.Arrow1`))
  (bind _returnvalue (`SceneComponent.K2_GetComponentLocation` (`self.CapsuleComponent`)))
  (bind (_returnvalue_roll _returnvalue_pitch) (`KismetMathLibrary.BreakRotator` (`SceneComponent.K2_GetComponentRotation` _capsulecomponent)))
  (bind (_returnvalue_roll_2 _returnvalue_pitch_2 _returnvalue_yaw) (`KismetMathLibrary.BreakRotator` (`KismetMathLibrary.FindLookAtRotation` (`SceneComponent.K2_GetComponentLocation` (`self.Mesh`)) (`self.K2_GetActorLocation` (`GameplayStatics.GetPlayerCharacter` 0)))))
  (set `self.Is Attacking` true)
  (`self.AI Stop`)
  (`KismetSystemLibrary.K2_SetTimerDelegate` (delegate `self.Attack`) 0.1 (`self.Looping`))
  (if (not (`self.IsDashing`))
    (`SceneComponent.K2_SetWorldRotation` _capsulecomponent (`KismetMathLibrary.MakeRotator` _returnvalue_roll _returnvalue_pitch _returnvalue_yaw) false false)
    (bind _result (`/Engine/EditorBlueprintResources/StandardMacros.IncrementInt` (`self.LoopCount`))
      (:`  `
        (if (not (<= _result 6))
          (set `self.Looping` false)
          (`/Engine/EditorBlueprintResources/StandardMacros.DoOnce` false :!label _label
            (:`Completed`
              (set `self.IsDashing` true)
              (bind _returnvalue_2 (`|SpawnActorFromClass` "/Game/Daniel/BP_ConeProjectile.BP_ConeProjectile_C" (`KismetMathLibrary.MakeTransform` (`SceneComponent.K2_GetComponentLocation` _arrow1) (`SceneComponent.K2_GetComponentRotation` _arrow1)) "AlwaysSpawn" "MultiplyWithRoot" null 3 self null))
              (`self.K2_AttachToComponent` _returnvalue_2 (`self.Arrow1`) "None" "SnapToTarget" "SnapToTarget" "KeepRelative" true)
              (`/Game/Design_Luke/Combat_Interface.Set Owner` _returnvalue_2 (`self.Mesh`) null self)
              (bind (_direction _float) (`Timeline|Timeline` :!via `PlayFromStart`)
                (:`Update`
                  (`SceneComponent.K2_SetWorldLocation` (`self.CapsuleComponent`) (`KismetMathLibrary.VLerp` _returnvalue (+ _returnvalue (* (`self.GetActorForwardVector`) 40.0)) _float) false false))
                (:`Finished`
                  (set `self.Is Attacking` false)
                  (set `self.LoopCount` 0)
                  (set `self.IsDashing` false)
                  (`self.K2_DestroyActor` _returnvalue_2)
                  (goto _label :!via `Reset`))))))))))

(fn `UserConstructionScript`
  (bind _returnvalue_location (`KismetMathLibrary.BreakTransform` (`SceneComponent.GetRelativeTransform` (`self.Mesh`))))
  (`parent.UserConstructionScript`)
  (bind _returnvalue (`AddComponent|NODE_AddSphereComponent-0` :`RelativeTransform` (`KismetMathLibrary.MakeTransform` _returnvalue_location)))
  (bind _output_get (set `self.Animation Detection ` _returnvalue))
  (`SphereComponent.SetSphereRadius` _output_get (`self.Animate Detection Range`) true)
  (`SphereComponent.SetSphereRadius` (`self.Max Range`) 400.0 true)
  (`SphereComponent.SetSphereRadius` (`self.Min Range`) 400.0 true))