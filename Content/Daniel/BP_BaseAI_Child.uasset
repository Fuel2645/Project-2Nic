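; BP_BaseAI_Child is an AI child Blueprint that moves only when an on-screen check against the first player controller passes.
; AIRun sets a looping 0.1-second timer, runs that check and, if not already moving, calls Movement with PlayerRef when valid or with no target otherwise.
; Perception updates from Player-class actors clear PlayerRef rather than storing the sensed actor.
; BeginPlay and construction only call the parent.
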(event `self.ReceiveBeginPlay`
  (`parent.ReceiveBeginPlay`))

(event `self.AIRun`
  (bind _playerref (`self.PlayerRef`))
  (`KismetSystemLibrary.K2_SetTimerDelegate` (delegate `self.AIRun`) 0.1 true)
  (bind _newparam2 (`self.CheckToSeeOnScreen` (`GameplayStatics.GetPlayerController` 0) self))
  (if _newparam2
    (if (not (`self.IsMoving`))
      (`/Engine/EditorBlueprintResources/StandardMacros.IsValid` _playerref
        (:`Is Valid`
          (`self.Movement` _playerref))
        (:`Is Not Valid`
          (`self.Movement` null))))))

(event `self.AIPerception.OnTargetPerceptionUpdated`
  (params (Actor :type "Actor Object Reference") (Stimulus :type "AIStimulus Structure"))
  (if (`KismetMathLibrary.ClassIsChildOf` (`GameplayStatics.GetObjectClass` Actor) "/Script/Engine.Player")
    (set `self.PlayerRef` null)))

(fn `UserConstructionScript`
  (`parent.UserConstructionScript`))