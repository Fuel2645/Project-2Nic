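; BP_Door is a locked door that opens when the interacting actor carries the required key.
; Interact searches the instigator's InventoryComponent for an item whose class matches KeyCheck, then prints a message and destroys the door.
; It creates a W_interact prompt on BeginPlay, and two box triggers show or hide it as the player character enters or leaves.
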(event `/Game/Luke_Dev/BPI_Interact.Interact`
  (params (Instigator :type "Character Object Reference"))
  (for _array_element (`/Game/Luke_Dev/InteractionSystem/InventoryComponent.Inventory` (`self.GetComponentByClass` Instigator "/Game/Luke_Dev/InteractionSystem/InventoryComponent.InventoryComponent_C"))
    (if (== (`.ItemClass_24_534652574CFB084F8949B3814DFA3472` (break `/Game/Luke_Dev/InteractionSystem/ItemInfo_S` _array_element)) (`self.KeyCheck`))
      (`KismetSystemLibrary.PrintString` "Door open")
      (`self.K2_DestroyActor`))))

(event `self.ReceiveBeginPlay`
  (bind _returnvalue (`|CreateWidget` "/Game/Roya/WidgetStuff/W_interact.W_interact_C" (`GameplayStatics.GetPlayerController` 0)))
  (set `self.Interact Widget` _returnvalue))

(event `self.Box1.OnComponentBeginOverlap`
  (params (OverlappedComponent :type "PrimitiveComponent Object Reference") (OtherActor :type "Actor Object Reference") (OtherComp :type "PrimitiveComponent Object Reference") (OtherBodyIndex :type Integer) (bFromSweep :type Boolean) (SweepResult :type "HitResult Structure (by ref)"))
  (if (== OtherActor (`GameplayStatics.GetPlayerCharacter` 0))
    (`UserWidget.AddToViewport` (`self.Interact Widget`) 0)))

(event `self.Box.OnComponentBeginOverlap`
  (params (OverlappedComponent :type "PrimitiveComponent Object Reference") (OtherActor :type "Actor Object Reference") (OtherComp :type "PrimitiveComponent Object Reference") (OtherBodyIndex :type Integer) (bFromSweep :type Boolean) (SweepResult :type "HitResult Structure (by ref)"))
  (if (== OtherActor (`GameplayStatics.GetPlayerCharacter` 0))
    (`UserWidget.AddToViewport` (`self.Interact Widget`) 0)))

(event `self.Box1.OnComponentEndOverlap`
  (params (OverlappedComponent :type "PrimitiveComponent Object Reference") (OtherActor :type "Actor Object Reference") (OtherComp :type "PrimitiveComponent Object Reference") (OtherBodyIndex :type Integer))
  (if (== OtherActor (`GameplayStatics.GetPlayerCharacter` 0))
    (`Widget.RemoveFromParent` (`self.Interact Widget`))))

(event `self.Box.OnComponentEndOverlap`
  (params (OverlappedComponent :type "PrimitiveComponent Object Reference") (OtherActor :type "Actor Object Reference") (OtherComp :type "PrimitiveComponent Object Reference") (OtherBodyIndex :type Integer))
  (if (== OtherActor (`GameplayStatics.GetPlayerCharacter` 0))
    (`Widget.RemoveFromParent` (`self.Interact Widget`))))

(fn `UserConstructionScript`)