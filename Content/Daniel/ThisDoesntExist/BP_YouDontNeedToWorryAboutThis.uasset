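; An interactable actor, apparently an Easter egg, that shows a hidden message when the player interacts with it nearby.
; Begin and end overlap events on a Box component set and clear a Help flag, reacting only to the first player's pawn.
; The Interact event prints the EasterStriing text on screen for a few seconds, but only while that flag is set.
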(event `/Game/Luke_Dev/BPI_Interact.Interact`
  (params (Instigator :type "Character Object Reference"))
  (if (`self.Help`)
    (`KismetSystemLibrary.PrintString` (`self.EasterStriing`) true true (struct :`G` 0.66 :`B` 1.0 :`A` 1.0) 5.0)))

(event `self.Box.OnComponentBeginOverlap`
  (params (OverlappedComponent :type "PrimitiveComponent Object Reference") (OtherActor :type "Actor Object Reference") (OtherComp :type "PrimitiveComponent Object Reference") (OtherBodyIndex :type Integer) (bFromSweep :type Boolean) (SweepResult :type "HitResult Structure (by ref)"))
  (if (== OtherActor (`GameplayStatics.GetPlayerPawn` 0))
    (set `self.Help` true)))

(event `self.Box.OnComponentEndOverlap`
  (params (OverlappedComponent :type "PrimitiveComponent Object Reference") (OtherActor :type "Actor Object Reference") (OtherComp :type "PrimitiveComponent Object Reference") (OtherBodyIndex :type Integer))
  (if (== (`GameplayStatics.GetPlayerPawn` 0) OtherActor)
    (set `self.Help` false)))

(fn `UserConstructionScript`)