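; BP_StopLooking is a trigger actor that reveals two static meshes and two point lights while the player is inside its box.
; On begin overlap with the player character, it moves both lights to fixed relative positions, sets their intensity, then unhides and shows all four components.
; On end overlap with the player pawn, it hides both meshes in game and dims the lights to zero intensity without hiding them.
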(event `self.Box.OnComponentBeginOverlap`
  (params (OverlappedComponent :type "PrimitiveComponent Object Reference") (OtherActor :type "Actor Object Reference") (OtherComp :type "PrimitiveComponent Object Reference") (OtherBodyIndex :type Integer) (bFromSweep :type Boolean) (SweepResult :type "HitResult Structure (by ref)"))
  (bind _pointlight (`self.PointLight`))
  (bind _pointlight1 (`self.PointLight1`))
  (bind _staticmesh1 (`self.StaticMesh1`))
  (if (== OtherActor (`GameplayStatics.GetPlayerCharacter` 0))
    (`SceneComponent.K2_SetRelativeLocation` _pointlight (-125.0 -105.0 282.0) false false)
    (`LightComponent.SetIntensity` _pointlight 80.0)
    (`SceneComponent.K2_SetRelativeLocation` _pointlight1 (113.0 65.0 282.0) false false)
    (`LightComponent.SetIntensity` _pointlight1 80.0)
    (`SceneComponent.SetHiddenInGame` _staticmesh1 false false)
    (`SceneComponent.SetHiddenInGame` (`self.PointLight1`) false false)
    (`SceneComponent.SetHiddenInGame` (`self.PointLight`) false false)
    (`SceneComponent.SetHiddenInGame` (`self.StaticMesh`) false false)
    (`SceneComponent.SetVisibility` _staticmesh1 true false)
    (`SceneComponent.SetVisibility` (`self.StaticMesh`) true false)
    (`SceneComponent.SetVisibility` (`self.PointLight`) true false)
    (`SceneComponent.SetVisibility` (`self.PointLight1`) true false)))

(event `self.Box.OnComponentEndOverlap`
  (params (OverlappedComponent :type "PrimitiveComponent Object Reference") (OtherActor :type "Actor Object Reference") (OtherComp :type "PrimitiveComponent Object Reference") (OtherBodyIndex :type Integer))
  (if (== OtherActor (`GameplayStatics.GetPlayerPawn` 0))
    (`SceneComponent.SetHiddenInGame` (`self.StaticMesh1`) true false)
    (`SceneComponent.SetHiddenInGame` (`self.StaticMesh`) true false)
    (`LightComponent.SetIntensity` (`self.PointLight`) 0.0)
    (`LightComponent.SetIntensity` (`self.PointLight1`) 0.0)))

(fn `UserConstructionScript`)