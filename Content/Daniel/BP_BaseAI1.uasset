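; Base AI character that patrols a looping list of points stored as offsets from its mesh's starting position.
; A 0.1-second timer starts movement only when the AI projects inside player 0's viewport, is idle and is in the Moving state.
; Movement can track a supplied actor instead, though the timer passes none.
; Events add or remove patrol points and stop movement; TakeDamage is an empty stub.
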(event `AIRun`
  (`KismetSystemLibrary.K2_SetTimerDelegate` (delegate `AIRun`) 0.1 true)
  (bind _newparam2 (`self.CheckToSeeOnScreen` (`GameplayStatics.GetPlayerController` 0) self))
  (if _newparam2
    (if (not (`self.IsMoving`))
      (switch `/Game/Daniel/AI_States` (`self.AI State`)
        (:`NewEnumerator1`
          (`self.Movement` null self))))))

(event `self.ReceiveBeginPlay`
  (`self.AIRun`))

(event `AI Stop`
  (`|AIMoveTo` self (`SceneComponent.K2_GetComponentLocation` (`self.Mesh`)) null
    (:`OnSuccess`
      (set `self.IsMoving` false))))

(event `Movement`
  (params (CharcterToMoveTo :type "Actor Object Reference") (`AI Ref` :type "Actor Object Reference"))
  (bind _returnvalue (`AIBlueprintHelperLibrary.GetAIController` `AI Ref`))
  (bind _patrol_points (`self.Patrol Points`))
  (bind _curentpatrolpoint (`self.CurentPatrolPoint`))
  (set `self.IsMoving` true)
  (`/Engine/EditorBlueprintResources/StandardMacros.IsValid` CharcterToMoveTo
    (:`Is Valid`
      (`AITask_MoveTo.AIMoveTo` _returnvalue (0.0 0.0 0.0) CharcterToMoveTo 100.0 "Default" "Enable" true true true
        (:`OnMoveFinished`
          (set `self.IsMoving` false))))
    (:`Is Not Valid`
      (`AITask_MoveTo.AIMoveTo` _returnvalue (+ (`|GetArrayItem` _patrol_points _curentpatrolpoint) (`self.StartingPos`)) null 10.0 "Default" "Enable" true true true
        (:`OnMoveFinished`
          (set `self.IsMoving` false)
          (if (== _curentpatrolpoint (`KismetArrayLibrary.Array_LastIndex` _patrol_points))
            (set `self.CurentPatrolPoint` 0)
            (else
              (`/Engine/EditorBlueprintResources/StandardMacros.IncrementInt` (`self.CurentPatrolPoint`)))))))))

(event `Take Damage`
  (params (DamageToTake :type Integer)))

(event `Add Patrol Point`
  (`KismetArrayLibrary.Array_Add` (`self.Patrol Points`) (50.0 50.0 10.0)))

(event `Remove Last Point`
  (bind _patrol_points (`self.Patrol Points`))
  (`KismetArrayLibrary.Array_Remove` _patrol_points (`KismetArrayLibrary.Array_LastIndex` _patrol_points)))

(event `Remove All Patrol Points`
  (bind _patrol_points (`self.Patrol Points`))
  (for (_ _array_index) _patrol_points :!label _label
    (`KismetArrayLibrary.Array_Remove` _patrol_points _array_index)
    (goto _label)))

(fn `CheckToSeeOnScreen`
  (params (NewParam :type "PlayerController Object Reference") (NewParam1 :type "Actor Object Reference"))
  (returns (NewParam2 :type Boolean))
  (bind (_returnvalue_x _returnvalue_y) (`KismetMathLibrary.BreakVector2D` (`WidgetLayoutLibrary.GetViewportSize`)))
  (bind _screenlocation (`PlayerController.ProjectWorldLocationToScreen` NewParam (`SceneComponent.K2_GetComponentLocation` (`Actor.RootComponent` NewParam1)) false))
  (return (and (> (`KismetMathLibrary.BreakVector2D` _screenlocation) 0.0) (< (`KismetMathLibrary.BreakVector2D` _screenlocation) _returnvalue_x) (> (`.Y` (`KismetMathLibrary.BreakVector2D` _screenlocation)) 0.0) (< (`.Y` (`KismetMathLibrary.BreakVector2D` _screenlocation)) _returnvalue_y))))

(fn `UserConstructionScript`
  (set `self.StartingPos` (`SceneComponent.K2_GetComponentLocation` (`self.Mesh`)))
  (for _ (`self.Patrol Points`)
    _))