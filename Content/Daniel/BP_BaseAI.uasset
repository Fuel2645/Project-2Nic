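; Base AI Blueprint that walks a looping patrol route while idle.
; The Construction Script stores the Mesh's world location as StartingPos, and PatrolPoints are offsets from it.
; Tick issues an AI MoveTo to the current point whenever IsIdle is set and no move is running, guarded by IsMoving.
; When the move finishes, the ArrowMove index advances and wraps back to the first point.
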(event `self.ReceiveTick`
  (params (DeltaSeconds :type "Float (single-precision)"))
  (bind _patrol_points (`self.Patrol Points`))
  (bind _arrowmove (`self.ArrowMove`))
  (if (`self.IsIdle`)
    (if (not (`self.IsMoving`))
      (`AITask_MoveTo.AIMoveTo` (`AIBlueprintHelperLibrary.GetAIController` self) (+ (`|GetArrayItem` _patrol_points _arrowmove) (`self.StartingPos`)) null 10.0 "Default" "Enable" true true true
        (:`then`
          (set `self.IsMoving` true))
        (:`OnMoveFinished`
          (set `self.IsMoving` false)
          (if (== _arrowmove (`KismetArrayLibrary.Array_LastIndex` _patrol_points))
            (set `self.ArrowMove` 0)
            (else
              (`/Engine/EditorBlueprintResources/StandardMacros.IncrementInt` (`self.ArrowMove`)))))))))

(fn `UserConstructionScript`
  (set `self.StartingPos` (`SceneComponent.K2_GetComponentLocation` (`self.Mesh`))))