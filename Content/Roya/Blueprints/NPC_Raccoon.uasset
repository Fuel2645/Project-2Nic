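; NPC_Raccoon is an interactable raccoon NPC that starts a conversation with whoever interacts with it.
; On Interact it runs the parent logic, stores the instigator and opens the conversation on its raccoon dialogue component.
; Interactable state, conversation close and construction only call the parent implementations.
; Leftover nodes for toggling mouse cursor and UI or game input modes are disconnected and never run.
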(event `/Game/Luke_Dev/BPI_Interact.Interact`
  (params (Instigator :type "Character Object Reference"))
  (`parent.Interact` Instigator)
  (set `self.InteractInstigator` Instigator)
  (`/Game/Roya/Blueprints/AC_DialogueBase.OpenConversation` (`self.AC_DialogueRaccoon`)))

(event `/Game/Luke_Dev/BPI_Interact.SetInteractableState`
  (params (CanShowInteract :type Boolean))
  (`parent.SetInteractableState` CanShowInteract))

(event `/Game/Luke_Dev/BPI_Interact.ConversationClosed`
  (`parent.ConversationClosed`))

(fn `UserConstructionScript`
  (`parent.UserConstructionScript`))