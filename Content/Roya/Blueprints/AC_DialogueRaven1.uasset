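; Dialogue component for the Raven1 NPC, an elderly-villager spirit who tells the player how they died peacefully of old age and miss their late spouse.
; It overrides the parent Dialogue function and switches on the dialogue tree index, with a single tree defined.
; Chained AddDialogue calls branch on state and chosen option, each offering one reply, and the last clears progress and closes the conversation.
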(fn `Dialogue`
  (`parent.Dialogue`)
  (switch `int` (`self.DialogueTreeIndex`)
    (:`0`
      (bind (_state _optionindex) (`self.AddDialogue` "Raven1" "Ah, another young one... it pains me to see so many who had their lives ahead of them end up in this place." (`|MakeArray` "How come you're the only one unharmed?" :!type "Text")))
      (switch `/Game/Roya/Blueprints/Enum_DialogueState` _state
        (:`NewEnumerator0`
          (switch `int` _optionindex
            (:`0`
              (bind (_state_2 _optionindex_2) (`self.AddDialogue` "Raven1" "The waking world was a dangerous place. So many of you adventurers met your demise during your travels - I lived a simple life in a small farming village by the sea. I wasn't poisoned or murdered; I didn't burn or starve. My days ended peacefully in my own bed... I simply grew old." (`|MakeArray` "Closing your eyes in your own bed and waking up here must have been quite the shock." :!type "Text")))
              (switch `/Game/Roya/Blueprints/Enum_DialogueState` _state_2
                (:`NewEnumerator0`
                  (switch `int` _optionindex_2
                    (:`0`
                      (bind _state_3 (`self.AddDialogue` "Raven1" "Oh it certainly was. My wife passed only a few days before myself; I was ready to be reunited with her in the next life. As far as I'm aware, she made it... I'm sure every day she wonders where I am. I miss her dearly." (`|MakeArray` "See you later." :!type "Text")))
                      (switch `/Game/Roya/Blueprints/Enum_DialogueState` _state_3
                        (:`NewEnumerator0`
                          (`self.ClearDialogueProgress`)
                          (`self.CloseConversation`))))))))))))))