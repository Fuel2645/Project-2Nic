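; AC_DialogueBear is the branching dialogue component for Bruin, who tells the player they are dead and trapped in the Forlorn Nexus.
; Its Dialogue function calls the parent version, then runs tree index 0 as nested AddDialogue calls that advance on each chosen option.
; A final choice asks about Stagcross village or the player's body, and both branches clear dialogue progress and close the conversation.
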(fn `Dialogue`
  (`parent.Dialogue`)
  (switch `int` (`self.DialogueTreeIndex`)
    (:`0`
      (bind (_state _optionindex) (`self.AddDialogue` "Bruin" "Hey kid, you got Rohan's ale delivery? He's just in the tavern up ahead. We were starting to think you'd gotten lost, the road from Lumena Village is pretty long, eh?" (`|MakeArray` "I'm sorry?" :!type "Text")))
      (switch `/Game/Roya/Blueprints/Enum_DialogueState` _state
        (:`NewEnumerator0`
          (switch `int` _optionindex
            (:`0`
              (bind (_state_2 _optionindex_2) (`self.AddDialogue` "Bruin" "Oh... you haven't come from Lumena, have you. I'm sorry, kid." (`|MakeArray` "Can you help me, please? I don't remember how I got here..." :!type "Text")))
              (switch `/Game/Roya/Blueprints/Enum_DialogueState` _state_2
                (:`NewEnumerator0`
                  (switch `int` _optionindex_2
                    (:`0`
                      (bind (_state_3 _optionindex_3) (`self.AddDialogue` "Bruin" "You're safe for now, kid, just try to calm yourself down. It might take you a while to adjust. Now, uh... where to begin... This realm doesn't look like home, does it? That's because it ain't. I'm sorry to have to be the one to break this news to you, but you're dead." (`|MakeArray` "Dead? Is... this the afterlife?" :!type "Text")))
                      (switch `/Game/Roya/Blueprints/Enum_DialogueState` _state_3
                        (:`NewEnumerator0`
                          (switch `int` _optionindex_3
                            (:`0`
                              (bind (_state_4 _optionindex_4) (`self.AddDialogue` "Bruin" "Well, that's where you were headed. It's where we were all headed. But this is no afterlife. This realm we're in, it lies just before it - those of us trapped here call it the Forlorn Nexus. Speak to Corvina; she'll tell you more. I ain't ever been very good at explaining this stuff to newcomers." (`|MakeArray` "What is this village?" "What's happened to my body?" :!type "Text")))
                              (switch `/Game/Roya/Blueprints/Enum_DialogueState` _state_4
                                (:`NewEnumerator0`
                                  (switch `int` _optionindex_4
                                    (:`0`
                                      (bind _state_5 (`self.AddDialogue` "Bruin" "This is Stagcross. We built this village centuries ago. It protects us from the creatures that roam the deep forest - and gives us some sense of home. You remember what home looks like, right? It was warm and comforting and safe... you'll find none of that in the Forlorn Nexus, so we had to make it ourselves. Keeps us sane." (`|MakeArray` "Goodbye." :!type "Text")))
                                      (switch `/Game/Roya/Blueprints/Enum_DialogueState` _state_5
                                        (:`NewEnumerator0`
                                          (`self.ClearDialogueProgress`)
                                          (`self.CloseConversation`))))
                                    (:`1`
                                      (bind _state_6 (`self.AddDialogue` "Bruin" "Those grizzly details will come back to you in time, as will the rest of your memory. Everyone here looks exactly how they did when they died - try not to stare too much. Some of us are quite a sight." (`|MakeArray` "Goodbye." :!type "Text")))
                                      (switch `/Game/Roya/Blueprints/Enum_DialogueState` _state_6
                                        (:`NewEnumerator0`
                                          (`self.ClearDialogueProgress`)
                                          (`self.CloseConversation`))))))))))))))))))))))