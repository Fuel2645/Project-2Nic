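; Dialogue component for Corvina, a Stagcross NPC who explains the Forlorn Nexus realm to newcomers sent over by Bruin.
; Overrides Dialogue, calls the parent, then switches on DialogueTreeIndex, with only the first tree defined.
; That tree chains three single-option AddDialogue nodes covering Lumena Village's library and the cathedral's history.
; The last reply clears dialogue progress and closes the conversation.
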(fn `Dialogue`
  (`parent.Dialogue`)
  (switch `int` (`self.DialogueTreeIndex`)
    (:`0`
      (bind (_state _optionindex) (`self.AddDialogue` "Corvina" "I saw you talking with Bruin. He sent you and your questions over here, right? He's always making me do the dirty work explaining this awful place to the newcomers. Says he's too 'sensitive'." (`|MakeArray` "How do you know so much about the Forlorn Nexus?" :!type "Text")))
      (switch `/Game/Roya/Blueprints/Enum_DialogueState` _state
        (:`NewEnumerator0`
          (switch `int` _optionindex
            (:`0`
              (bind (_state_2 _optionindex_2) (`self.AddDialogue` "Corvina" "I wandered the forests and mountains alone when I first awoke here, it could have lasted months or years, I couldn't tell you. Eventually, I stumbled across Lumena Village. It's quite a long way from Stagcross. The special thing about Lumena is its library. The village's founders were scholars, so all the knowledge they've collected about this realm over time is stored there. Not much else to do but read." (`|MakeArray` "Why build a place of worship if we're all dead already?" :!type "Text")))
              (switch `/Game/Roya/Blueprints/Enum_DialogueState` _state_2
                (:`NewEnumerator0`
                  (switch `int` _optionindex_2
                    (:`0`
                      (bind _state_3 (`self.AddDialogue` "Corvina" "The cathedral was the first building to be completed in Stagcross. Our only hope is prayer - perhaps, if we pray loud enough, the Gods will hear our calls and rescue us from this cursed realm, allowing our souls to move on to the afterlife where they belong. That's what we thought in the early days, at least. It's been centuries, and still, no salvation. People don't visit the cathedral as much as they used to." (`|MakeArray` "Thanks, Corvina." :!type "Text")))
                      (switch `/Game/Roya/Blueprints/Enum_DialogueState` _state_3
                        (:`NewEnumerator0`
                          (`self.ClearDialogueProgress`)
                          (`self.CloseConversation`))))))))))))))