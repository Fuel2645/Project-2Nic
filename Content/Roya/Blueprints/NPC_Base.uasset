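; NPC_Base is a base NPC Blueprint providing a floating character name, an interact prompt and dialogue input handling.
; Player overlap with the capsule adds or removes the W_interact widget created on BeginPlay.
; Interact switches input to UI-only, focused on the ACDialogueBase dialogue widget; ConversationClosed notifies the instigator and restores game-only input.
; SetInteractableState toggles the name text and mouse cursor; the construction script fills in the name.
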(event `/Game/Luke_Dev/BPI_Interact.Interact`
  (params (Instigator :type "Character Object Reference"))
  (bind _returnvalue (`GameplayStatics.GetPlayerController` 0))
  (set `PlayerController.bShowMouseCursor` true _returnvalue)
  (`WidgetBlueprintLibrary.SetInputMode_UIOnlyEx` _returnvalue (`/Game/Roya/Blueprints/AC_DialogueBase.DialogueWidget` (`self.AC_DialogueBase`))))

(event `/Game/Luke_Dev/BPI_Interact.SetInteractableState`
  (params (CanShowInteract :type Boolean))
  (bind _returnvalue (`GameplayStatics.GetPlayerController` 0))
  (if CanShowInteract
    (`SceneComponent.SetVisibility` (`self.txt_CharacterName`) true false)
    (set `PlayerController.bShowMouseCursor` true _returnvalue)
    (else
      (`SceneComponent.SetVisibility` (`self.txt_CharacterName`) false false)
      (set `PlayerController.bShowMouseCursor` false _returnvalue))))

(event `/Game/Luke_Dev/BPI_Interact.ConversationClosed`
  (bind _returnvalue (`GameplayStatics.GetPlayerController` 0))
  (message `/Game/Luke_Dev/BPI_Interact.ConversationClosed` (`self.InteractInstigator`))
  (`WidgetBlueprintLibrary.SetInputMode_GameOnly` _returnvalue)
  (set `PlayerController.bShowMouseCursor` false _returnvalue))

(event `self.CapsuleComponent.OnComponentBeginOverlap`
  (params (OverlappedComponent :type "PrimitiveComponent Object Reference") (OtherActor :type "Actor Object Reference") (OtherComp :type "PrimitiveComponent Object Reference") (OtherBodyIndex :type Integer) (bFromSweep :type Boolean) (SweepResult :type "HitResult Structure (by ref)"))
  (if (== OtherActor (`GameplayStatics.GetPlayerCharacter` 0))
    (`UserWidget.AddToViewport` (`self.InteractPrompt`) 0)))

(event `self.CapsuleComponent.OnComponentEndOverlap`
  (params (OverlappedComponent :type "PrimitiveComponent Object Reference") (OtherActor :type "Actor Object Reference") (OtherComp :type "PrimitiveComponent Object Reference") (OtherBodyIndex :type Integer))
  (if (== (`GameplayStatics.GetPlayerCharacter` 0) OtherActor)
    (`Widget.RemoveFromParent` (`self.InteractPrompt`))))

(event `self.ReceiveBeginPlay`
  (bind _returnvalue (`|CreateWidget` "/Game/Roya/WidgetStuff/W_interact.W_interact_C"))
  (set `self.InteractPrompt` _returnvalue))

(fn `UserConstructionScript`
  (`TextRenderComponent.K2_SetText` (`self.txt_CharacterName`) (`self.CharacterName`)))