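; Dialogue component for Rohan, a drink server who gives the player the quest to clear the catacombs and investigate the castle, pointing them to Harvey in the graveyard.
; It overrides Dialogue, calls the parent, then switches on DialogueTreeIndex, with only tree 0 filled in.
; That tree is a linear chain of five nested AddDialogue calls with one reply each, ending by clearing dialogue progress and closing the conversation.
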(fn `Dialogue`
  (`parent.Dialogue`)
  (switch `int` (`self.DialogueTreeIndex`)
    (:`0`
      (bind (_state _optionindex) (`self.AddDialogue` "Rohan" "Sorry if you talk to Willow. She's always like that, although I can't really blame her. What can I get for you? I'm afraid your options are limited, as it seems the courier from Lumena Village has met a dour fate. It'll be months before the next ale delivery. No idea how Willow will cope." (`|MakeArray` "I'm not looking for a drink. I'm still trying to wrap my head around this place." :!type "Text")))
      (switch `/Game/Roya/Blueprints/Enum_DialogueState` _state
        (:`NewEnumerator0`
          (switch `int` _optionindex
            (:`0`
              (bind _state_2 (`self.AddDialogue` "Rohan" "Ah, I understand. My condolences. You seem like the adventuring type - how about I offer you something other than a drink. Something far more difficult to come across in this world." (`|MakeArray` "I'm listening." :!type "Text")))
              (switch `/Game/Roya/Blueprints/Enum_DialogueState` _state_2
                (:`NewEnumerator0`
                  (switch `int` 0
                    (:`0`
                      (bind (_state_3 _optionindex_2) (`self.AddDialogue` "Rohan" "A sense of purpose. This village has a problem, however none of us are exactly qualified to solve it. In the graveyard beyond the village lies the entrance to the catacombs, and they're crawling with monsters. Usually they stay put, but recently some of them have been escaping. Our groundskeeper Harvey is a confident fighter, but it has become too much for him to bear alone." (`|MakeArray` "You need me to clear out the catacombs." :!type "Text")))
                      (switch `/Game/Roya/Blueprints/Enum_DialogueState` _state_3
                        (:`NewEnumerator0`
                          (switch `int` _optionindex_2
                            (:`0`
                              (bind (_state_4 _optionindex_3) (`self.AddDialogue` "Rohan" "We do, yes, but there's another thing. The castle atop the cliffside was abandoned by its founders long ago - and the same day those monsters started escaping, we noticed faint candlelight flickering in the castle windows. Someone, or something, is in there, and I think it's the reason the monsters have become more active." (`|MakeArray` "How do I get into the castle?" :!type "Text")))
                              (switch `/Game/Roya/Blueprints/Enum_DialogueState` _state_4
                                (:`NewEnumerator0`
                                  (switch `int` _optionindex_3
                                    (:`0`
                                      (bind _state_5 (`self.AddDialogue` "Rohan" "Speak with Harvey in the graveyard, he'll explain more. This is quite the dangerous expedition you're undertaking, stranger. You have my thanks, and should you be successful, you have drinks on the house." (`|MakeArray` "I'm on it." :!type "Text")))
                                      (switch `/Game/Roya/Blueprints/Enum_DialogueState` _state_5
                                        (:`NewEnumerator0`
                                          (`self.ClearDialogueProgress`)
                                          (`self.CloseConversation`))))))))))))))))))))))