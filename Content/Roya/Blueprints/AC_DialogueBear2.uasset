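; Dialogue component for the NPC Harvey, who warns the player about the graveyard crypts and explains that the castle key is locked inside them.
; Overrides Dialogue, calls the parent, then switches on DialogueTreeIndex, with only the first tree populated.
; That tree chains four AddDialogue calls, each with one reply, advancing on Pass Through and option index.
; The final reply clears dialogue progress and closes the conversation.
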(fn `Dialogue`
  (`parent.Dialogue`)
  (switch `int` (`self.DialogueTreeIndex`)
    (:`0`
      (bind (_state _optionindex) (`self.AddDialogue` "Harvey" "Careful round here, stranger, I'd hate to see you become one of those things." (`|MakeArray` "Become one?" :!type "Text")))
      (switch `/Game/Roya/Blueprints/Enum_DialogueState` _state
        (:`NewEnumerator0`
          (switch `int` _optionindex
            (:`0`
              (bind (_state_2 _optionindex_2) (`self.AddDialogue` "Harvey" "That's where they come from. Some souls just aren't strong enough to handle existence in this realm, and it drives them insane. For the safety of those of us who can hang on, we have to lock them down in the crypt. What are you doing here, anyway? I told Rohan to warn newcomers against the graveyard." (`|MakeArray` "I'm here to stop them escaping. Permenantly." :!type "Text")))
              (switch `/Game/Roya/Blueprints/Enum_DialogueState` _state_2
                (:`NewEnumerator0`
                  (switch `int` _optionindex_2
                    (:`0`
                      (bind (_state_3 _optionindex_3) (`self.AddDialogue` "Harvey" "That's quite the claim. But if Rohan saw something in you, then I trust you can handle yourself. I'm guessing he's told you about the castle - I'm afraid it won't be as simple as walking in and quelling whatever has set up shop in there. The castle key was locked in the crypts by its founders shortly after they abandoned it. Couldn't tell you why." (`|MakeArray` "Looks like I have my work cut out for me." :!type "Text")))
                      (switch `/Game/Roya/Blueprints/Enum_DialogueState` _state_3
                        (:`NewEnumerator0`
                          (switch `int` _optionindex_3
                            (:`0`
                              (bind _state_4 (`self.AddDialogue` "Harvey" "You certainly do. Allow me to offer my thanks. I'm a fighter, but I'm not what I used to be. A crafty adventurer like yourself would fare far better down there than I ever could. Plus, someone has to stay up top and keep the villagers safe." (`|MakeArray` "I'll see you soon, Harvey." :!type "Text")))
                              (switch `/Game/Roya/Blueprints/Enum_DialogueState` _state_4
                                (:`NewEnumerator0`
                                  (`self.ClearDialogueProgress`)
                                  (`self.CloseConversation`))))))))))))))))))