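; Player character with limb-based health, swappable socket-mounted weapons, charged attacks, dash, sprint, stamina and enemy lock-on.
; Body-part overlaps pass projectile hits to the BPCHP component, with timed invulnerability on damage, bone hiding for lost limbs and respawn at spawn location.
; Attack input charges while held and releases through the current weapon.
; Lock-on sphere-traces for an enemy, and a camera box trace handles transparent materials on obstructing meshes.
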(event `self.ReceiveBeginPlay`
  (bind _bpc_hp (`self.BPC_HP`))
  (bind (_returnvalue_location _returnvalue_rotation) (`KismetMathLibrary.BreakTransform` (`SceneComponent.GetSocketTransform` (`self.Mesh`) "Weapon_Sock" "RTS_World")))
  (`|ExecutionSequence`
    (:`then_0`
      (message `EnhancedInputSubsystemInterface.AddMappingContext` (pcsubsystem `EnhancedInputLocalPlayerSubsystem` (`GameplayStatics.GetPlayerController` 0)) "/Game/Design_Luke/Test_Inputs/D_Luke_Move+Combat_MappingTest.D_Luke_Move+Combat_MappingTest" 0 (struct))
      ;[1 0 0] Create Bar Widgets
      (bind _returnvalue (`|CreateWidget` "/Game/Andy_B1106369/Ui/Health_Stamina_Bar/WB_Health_Stamina.WB_Health_Stamina_C"))
      (bind _output_get (set `self.HUD_Widget_HP&Stam` _returnvalue))
      (`UserWidget.AddToViewport` _output_get 0)
      (`KismetSystemLibrary.PrintString` "Hello")
      ;[1 0 0] Set Health
      (bind _output_get_2 (set `self.Current_Health_Head` (`BlueprintMapLibrary.Map_Find` (`/Game/Design_Luke/BPC_HP.Health_Pools` _bpc_hp) (`|GetArrayItem` (`/Game/Design_Luke/BPC_HP.LimbNames` _bpc_hp)))))
      (message `/Game/Andy_B1106369/Ui/Widget_interface.Update Health` (`self.HUD_Widget_HP&Stam`) _output_get_2 "None"))
    (:`then_2`
      ;[1 0 0.9314] Equip Weapon
      (if (`self.HoldingWeapon`)
        (bind _returnvalue_2 (`|SpawnActorFromClass` (`BlueprintMapLibrary.Map_Find` (`self.Equipment`) (`self.Selected`)) (`KismetMathLibrary.MakeTransform` _returnvalue_location _returnvalue_rotation (2.0 2.0 2.0)) "Undefined" "MultiplyWithRoot" null null))
        (bind _output_get_3 (set `self.CurrentWeapon` _returnvalue_2))
        (message `/Game/Design_Luke/Combat_Interface.Set Owner` _output_get_3 (`self.Mesh`) (`self.WeaponArm`) self)))))

(event `EnhancedInput|/Game/Design_Luke/Test_Inputs/Individual_InputTest/IA_Cycle`
  (params (ActionValue :type "Float (double-precision)") (ElapsedSeconds :type "Float (double-precision)") (TriggeredSeconds :type "Float (double-precision)") (InputAction :type "InputAction Object Reference" :default "/Game/Design_Luke/Test_Inputs/Individual_InputTest/IA_Cycle.IA_Cycle"))
  ;[1 0 0.9087] Cycle Weapons
  (:`Started`
    (`self.CycleWeapons` (`KismetMathLibrary.FTrunc` ActionValue))))

(event `EnhancedInput|/Game/Design_Luke/Test_Inputs/Individual_InputTest/IA_CombatAtk`
  (params (ActionValue :type Boolean) (ElapsedSeconds :type "Float (double-precision)") (TriggeredSeconds :type "Float (double-precision)") (InputAction :type "InputAction Object Reference" :default "/Game/Design_Luke/Test_Inputs/Individual_InputTest/IA_CombatAtk.IA_CombatAtk"))
  (bind _bpc_hp (`self.BPC_HP`))
  (bind _limbactive (`/Game/Design_Luke/BPC_HP.LimbActiveCheck` _bpc_hp (`|GetArrayItem` (`/Game/Design_Luke/BPC_HP.LimbNames` _bpc_hp) 2)))
  (:`Triggered`
    (if _limbactive
      ;[1 1 1] Charge Attack whil
      (`/Engine/EditorBlueprintResources/StandardMacros.DoOnce` false :!label _label
        (:`Completed`
          (bind _output_get (set `self.Charging` true))
          (`KismetSystemLibrary.Delay` 1.5 :!label _label_2)
          (if _output_get
            (`/Engine/EditorBlueprintResources/StandardMacros.IncrementFloat` (`self.AttackCharged`)
              (:`  `
                (bind (_black_dmg _red_dmg _orange_dmg _green_dmg) (`/Game/Design_Luke/BPC_HP.CheckDmgColours` (`self.BPC_HP`)))
                (message `/Game/Design_Luke/Combat_Interface.Impact Feedback` (`self.CurrentWeapon`) null _black_dmg _red_dmg _orange_dmg _green_dmg (`self.AttackCharged`))
                (goto _label_2))))))))
  (:`Completed`
    (if _limbactive
      (`|ExecutionSequence`
        (:`then_0`
          (set `self.Charging` false)
          (if (`self.HoldingWeapon`)
            (message `/Game/Design_Luke/Combat_Interface.ReleaseAtk` (`self.CurrentWeapon`) (`self.AttackCharged`))
            (`KismetSystemLibrary.PrintString` (`KismetStringLibrary.Concat_StrStr` "atk " "dmg = " (`KismetStringLibrary.Conv_DoubleToString` (`self.AttackCharged`))))
            (set `self.AttackCharged` 1.0)
            (else
              (set `self.CurrentWeapon` self))))
        (:`then_1`
          (goto _label :!via `Reset`)))
      (else
        (goto _label :!via `Reset`)))))

(event `/Game/Design_Luke/Combat_Interface.Launch Projectile`
  (params (UseProjectile :type "/Game/Design_Luke/ProjectileChildren/RangedAttacks/BP_Ranged_ProjectileParent Class Reference") (Dmg :type "Float (double-precision)"))
  (bind _returnvalue (+ (`SceneComponent.GetSocketLocation` (`self.WeaponArm`) "None") (`self.ProjectileOffset`)))
  ;[1 0.1277 0.8524] Launch Weapon Projectile
  (`/Engine/EditorBlueprintResources/StandardMacros.DoOnce` false :!label _label_3
    (:`Completed`
      (`|SpawnActorFromClass` "/Game/Design_Luke/ProjectileChildren/RangedAttacks/BP_Bolt_Projectile_Child.BP_Bolt_Projectile_Child_C" (`KismetMathLibrary.MakeTransform` _returnvalue (`self.K2_GetActorRotation`) (2.0 2.0 2.0)) "AlwaysSpawn" "OverrideRootScale" null (`self.AttackCharged`) self null)
      (`GameplayStatics.PlaySoundAtLocation` "/Game/Daniel/reverb-fart-sound-effect-hd-+-download-made-with-Voicemod.reverb-fart-sound-effect-hd-+-download-made-with-Voicemod" _returnvalue (struct) 1.0 1.0 0.0 null null null null) ; Play firing sound
      (`KismetSystemLibrary.Delay` 0.5)
      (goto _label_3 :!via `Reset`))))

(event `Key|One`
  (params (Key :type "Key Structure"))
  (bind _health_pools (`/Game/Design_Luke/BPC_HP.Health_Pools` (`self.BPC_HP`)))
  (:`Pressed`
    (`BlueprintMapLibrary.Map_Add` _health_pools "Head" 2.0))
  (:`Released`
    (`BlueprintMapLibrary.Map_Add` _health_pools "Head" 3.0)))

(event `Key|LeftMouseButton`
  (params (Key :type "Key Structure")))

(event `EnhancedInput|/Game/Design_Luke/Test_Inputs/Individual_InputTest/IA_Vertical_LB_Test`
  (params (ActionValue :type "Float (double-precision)") (ElapsedSeconds :type "Float (double-precision)") (TriggeredSeconds :type "Float (double-precision)") (InputAction :type "InputAction Object Reference" :default "/Game/Design_Luke/Test_Inputs/Individual_InputTest/IA_Vertical_LB_Test.IA_Vertical_LB_Test"))
  ;[1 0.8342 0] Move
  (:`Triggered`
    (`self.AddMovementInput` (0.5 0.5 0.0) ActionValue)))

(event `EnhancedInput|/Game/Design_Luke/Test_Inputs/Individual_InputTest/IA_Turn`
  (params (ActionValue :type "Vector2D Structure") (ElapsedSeconds :type "Float (double-precision)") (TriggeredSeconds :type "Float (double-precision)") (InputAction :type "InputAction Object Reference" :default "/Game/Design_Luke/Test_Inputs/Individual_InputTest/IA_Turn.IA_Turn"))
  ;[1 1 1] evidence for learning
)

(event `EnhancedInput|/Game/Design_Luke/Test_Inputs/Individual_InputTest/IA_Horizontal_LB_Test`
  (params (ActionValue :type "Float (double-precision)") (ElapsedSeconds :type "Float (double-precision)") (TriggeredSeconds :type "Float (double-precision)") (InputAction :type "InputAction Object Reference" :default "/Game/Design_Luke/Test_Inputs/Individual_InputTest/IA_Horizontal_LB_Test.IA_Horizontal_LB_Test"))
  ;[1 0.8342 0] Move
  (:`Triggered`
    (`self.AddMovementInput` (-0.5 0.5 0.0) ActionValue)))

(event `self.ReceiveTick`
  (params (DeltaSeconds :type "Float (single-precision)"))
  ;[1 1 1] Lock
  (`|ExecutionSequence`
    (:`then_0`
      (if (`self.LockOn?`)
        (`self.K2_SetActorRotation` (`KismetMathLibrary.MakeRotator` (.roll (`KismetMathLibrary.RInterpTo` (`self.K2_GetActorRotation`) (`KismetMathLibrary.FindLookAtRotation` (`self.K2_GetActorLocation`) (`KismetMathLibrary.MakeVector` (.x (`self.K2_GetActorLocation` (`self.TargetEnemy(LockedOn)`))) (.y (`self.K2_GetActorLocation` (`self.TargetEnemy(LockedOn)`))) (- (.z (`self.K2_GetActorLocation` (`self.TargetEnemy(LockedOn)`))) 20.0))) (`GameplayStatics.GetWorldDeltaSeconds`) 4.0)) (.pitch (`KismetMathLibrary.RInterpTo` (`self.K2_GetActorRotation`) (`KismetMathLibrary.FindLookAtRotation` (`self.K2_GetActorLocation`) (`KismetMathLibrary.MakeVector` (.x (`self.K2_GetActorLocation` (`self.TargetEnemy(LockedOn)`))) (.y (`self.K2_GetActorLocation` (`self.TargetEnemy(LockedOn)`))) (- (.z (`self.K2_GetActorLocation` (`self.TargetEnemy(LockedOn)`))) 20.0))) (`GameplayStatics.GetWorldDeltaSeconds`) 4.0)) (.yaw (`KismetMathLibrary.RInterpTo` (`self.K2_GetActorRotation`) (`KismetMathLibrary.FindLookAtRotation` (`self.K2_GetActorLocation`) (`KismetMathLibrary.MakeVector` (.x (`self.K2_GetActorLocation` (`self.TargetEnemy(LockedOn)`))) (.y (`self.K2_GetActorLocation` (`self.TargetEnemy(LockedOn)`))) (- (.z (`self.K2_GetActorLocation` (`self.TargetEnemy(LockedOn)`))) 20.0))) (`GameplayStatics.GetWorldDeltaSeconds`) 4.0))))
        (set `CharacterMovementComponent.bOrientRotationToMovement` false (`self.CharacterMovement`))))))

(event `EnhancedInput|/Game/Daniel_A/Input/Actions/IA_Dash`
  (params (ActionValue :type Boolean) (ElapsedSeconds :type "Float (double-precision)") (TriggeredSeconds :type "Float (double-precision)") (InputAction :type "InputAction Object Reference" :default "/Game/Daniel_A/Input/Actions/IA_Dash.IA_Dash"))
  (bind (_velocity_x _velocity_y _velocity_z) (`KismetMathLibrary.BreakVector` (`MovementComponent.Velocity` (`self.CharacterMovement`))))
  ;[1 1 1] Dash/Sprint
  (:`Triggered`
    (`self.StartSprinting`))
  (:`Started`
    (if (> (`self.Stamina`) 100.0)
      (set `self.isDashing` true)
      (bind (_direction _distance) (`Timeline|Timeline` :!via `PlayFromStart`)
        (:`Update`
          (bind (_returnvalue_x _returnvalue_y) (`KismetMathLibrary.BreakVector` (* (`self.GetActorForwardVector`) (* _distance (`self.Dash Distance`)))))
          (set `MovementComponent.Velocity` (`KismetMathLibrary.MakeVector` _returnvalue_x _returnvalue_y _velocity_z) (`self.CharacterMovement`))
          (if (`|GetInputActionValue`)
            (`self.StartSprinting`)))
        (:`Finished`
          (set `self.isDashing` false)
          (if (not (`|GetInputActionValue`))
            (set `self.Stamina` (`KismetMathLibrary.Clamp` (- (`self.Stamina`) 100) 0 (`self.Max Stamina`)))
            (`KismetSystemLibrary.PrintString` (`KismetStringLibrary.Conv_IntToString` (`self.Stamina`))))))))
  (:`Completed`
    (`self.StopSprinting`)))

(event `EnhancedInput|/Game/Daniel_A/Input/Actions/IA_Sprint`
  (params (ActionValue :type Boolean) (ElapsedSeconds :type "Float (double-precision)") (TriggeredSeconds :type "Float (double-precision)") (InputAction :type "InputAction Object Reference" :default "/Game/Daniel_A/Input/Actions/IA_Sprint.IA_Sprint"))
  ;[0.05098 0.05098 0.05098] Sprinting
  (:`Triggered`
    (`self.StartSprinting`))
  (:`Completed`
    (`self.StopSprinting`)))

(event `/Game/Design_Luke/Combat_Interface.Die`
  ;[0 0 0] Die
  (`KismetSystemLibrary.PrintString` "died")
  (`SceneComponent.K2_SetWorldLocation` (`self.CapsuleComponent`) (`self.SpawnLocation`) false false))

(event `/Game/Design_Luke/Combat_Interface.Impact Feedback`
  (params (Trigger :type "Actor Object Reference") (Black_Dmg :type "Float (double-precision)") (Red_Dmg :type "Float (double-precision)") (Orange_Dmg :type "Float (double-precision)") (Green_Dmg :type "Float (double-precision)") (Dmg :type "Float (double-precision)"))
  ;[0.02022 0 1] Spawned Projectiles Feedback
  (bind (_black_dmg _red_dmg _orange_dmg _green_dmg) (`/Game/Design_Luke/BPC_HP.CheckDmgColours` (`self.BPC_HP`)))
  (message `/Game/Design_Luke/Combat_Interface.Impact Feedback` Trigger null _black_dmg _red_dmg _orange_dmg _green_dmg 0.0))

(event `/Game/Design_Luke/Combat_Interface.Stagger`
  ;[0.9883 0.5619 1] Stagger
  (`/Engine/EditorBlueprintResources/StandardMacros.DoOnce` false))

(event `StaminaDrain`
  (bind _stamina (`self.Stamina`))
  ;[1 1 1] Stamina Drain/Regen
  (bind _output_get (set `self.Stamina` (`KismetMathLibrary.Clamp` (- (`self.Stamina`) 1) 0 (`self.Max Stamina`))))
  (if (== _output_get 0)
    (`self.StopSprinting`)
    (elif (`self.isSprinting`)
      (`KismetSystemLibrary.Delay` 0.1)
      (`self.StaminaDrain`)
      (`KismetSystemLibrary.PrintString` (`KismetStringLibrary.Conv_IntToString` _stamina) true true (struct :`G` 0.66 :`B` 1.0 :`A` 1.0) 0.1)
      (`self.Update Stamina` (`KismetMathLibrary.Conv_IntToDouble` _stamina)))))

(event `self.Torso.OnComponentBeginOverlap`
  (params (OverlappedComponent :type "PrimitiveComponent Object Reference") (OtherActor :type "Actor Object Reference") (OtherComp :type "PrimitiveComponent Object Reference") (OtherBodyIndex :type Integer) (bFromSweep :type Boolean) (SweepResult :type "HitResult Structure (by ref)"))
  (bind _bpc_hp (`self.BPC_HP`))
  ;[0.357 1 0.07456] Torso
  (`/Engine/EditorBlueprintResources/StandardMacros.DoOnce` false :!label _label_4
    (:`Completed`
      (if (and (`KismetMathLibrary.ClassIsChildOf` (`GameplayStatics.GetObjectClass` OtherActor) "/Game/Design_Luke/ProjectileChildren/BP_ParentProjectile.BP_ParentProjectile_C") (`BlueprintMapLibrary.Map_Find` (`/Game/Design_Luke/BPC_HP.Active_Limbs` _bpc_hp) (`|GetArrayItem` (`/Game/Design_Luke/BPC_HP.LimbNames` _bpc_hp))))
        (message `/Game/Design_Luke/Combat_Interface.Hit_by_Atk` OtherActor 0.0 self "Torso" (`self.BPC_HP`))
        (goto _label_4 :!via `Reset`)
        (else
          (goto _label_4 :!via `Reset`))))))

(event `self.R_Arm_Box.OnComponentBeginOverlap`
  (params (OverlappedComponent :type "PrimitiveComponent Object Reference") (OtherActor :type "Actor Object Reference") (OtherComp :type "PrimitiveComponent Object Reference") (OtherBodyIndex :type Integer) (bFromSweep :type Boolean) (SweepResult :type "HitResult Structure (by ref)"))
  (bind _bpc_hp (`self.BPC_HP`))
  (bind _output (`|GetArrayItem` (`/Game/Design_Luke/BPC_HP.LimbNames` _bpc_hp) 2))
  ;[0.357 1 0.07456] Right Limb
  (`/Engine/EditorBlueprintResources/StandardMacros.DoOnce` false :!label _label_5
    (:`Completed`
      (if (and (`KismetMathLibrary.ClassIsChildOf` (`GameplayStatics.GetObjectClass` OtherActor) "/Game/Design_Luke/ProjectileChildren/BP_ParentProjectile.BP_ParentProjectile_C") (`BlueprintMapLibrary.Map_Find` (`/Game/Design_Luke/BPC_HP.Active_Limbs` _bpc_hp) _output))
        (message `/Game/Design_Luke/Combat_Interface.Hit_by_Atk` OtherActor 0.0 self _output (`self.BPC_HP`))
        (goto _label_5 :!via `Reset`)
        (else
          (goto _label_5 :!via `Reset`))))))

(event `StaminaRegen`
  (bind _stamina (`self.Stamina`))
  ;[1 1 1] Stamina Drain/Regen
  (bind _output_get (set `self.Stamina` (`KismetMathLibrary.Clamp` (+ (`self.Stamina`) 2) 0 (`self.Max Stamina`))))
  (if (== _output_get (`self.Max Stamina`))
    _
    (elif (not (`self.isSprinting`))
      (`KismetSystemLibrary.Delay` 0.1)
      (`self.StaminaRegen`)
      (`KismetSystemLibrary.PrintString` (`KismetStringLibrary.Conv_IntToString` _stamina) true true (struct :`G` 0.66 :`B` 1.0 :`A` 1.0) 0.1)
      (`self.Update Stamina` (`KismetMathLibrary.Conv_IntToDouble` _stamina)))))

(event `self.Head_Sphere.OnComponentBeginOverlap`
  (params (OverlappedComponent :type "PrimitiveComponent Object Reference") (OtherActor :type "Actor Object Reference") (OtherComp :type "PrimitiveComponent Object Reference") (OtherBodyIndex :type Integer) (bFromSweep :type Boolean) (SweepResult :type "HitResult Structure (by ref)"))
  (bind _bpc_hp (`self.BPC_HP`))
  ;[0.357 1 0.07456] Head
  (`/Engine/EditorBlueprintResources/StandardMacros.DoOnce` false :!label _label_6
    (:`Completed`
      (if (and (`KismetMathLibrary.ClassIsChildOf` (`GameplayStatics.GetObjectClass` OtherActor) "/Game/Design_Luke/ProjectileChildren/BP_ParentProjectile.BP_ParentProjectile_C") (`BlueprintMapLibrary.Map_Find` (`/Game/Design_Luke/BPC_HP.Active_Limbs` _bpc_hp) (`|GetArrayItem` (`/Game/Design_Luke/BPC_HP.LimbNames` _bpc_hp))))
        (message `/Game/Design_Luke/Combat_Interface.Hit_by_Atk` OtherActor 0.0 self "Head" (`self.BPC_HP`))
        (goto _label_6 :!via `Reset`)
        (else
          (goto _label_6 :!via `Reset`))))))

(event `/Game/Design_Luke/Combat_Interface.LoseLimb`
  (params (LimbName :type Name))
  ;[0.005208 0.005208 0.005208] Limb test
  (`self.HideBone` LimbName))

(event `Key|R`
  (params (Key :type "Key Structure"))
  (bind _bpc_hp (`self.BPC_HP`))
  (bind _active_limbs (`/Game/Design_Luke/BPC_HP.Active_Limbs` _bpc_hp))
  (bind _health_pools (`/Game/Design_Luke/BPC_HP.Health_Pools` _bpc_hp))
  ;[0.005208 0.005208 0.005208] Limb test
  (:`Pressed`
    (if (`BlueprintMapLibrary.Map_Find` _active_limbs "Elbow_Right")
      (`self.HideBone` "Elbow_Right")
      (`BlueprintMapLibrary.Map_Add` _active_limbs "Elbow_Right")
      (`BlueprintMapLibrary.Map_Add` _health_pools "Elbow_Right" 4.0)
      (else
        (`self.UnHideBone` "Elbow_Right")
        (`BlueprintMapLibrary.Map_Add` _active_limbs "Elbow_Right" true)
        (`BlueprintMapLibrary.Map_Add` _health_pools "Elbow_Right" 4.0)))))

(event `self.L_Arm_Box.OnComponentBeginOverlap`
  (params (OverlappedComponent :type "PrimitiveComponent Object Reference") (OtherActor :type "Actor Object Reference") (OtherComp :type "PrimitiveComponent Object Reference") (OtherBodyIndex :type Integer) (bFromSweep :type Boolean) (SweepResult :type "HitResult Structure (by ref)"))
  (bind _bpc_hp (`self.BPC_HP`))
  (bind _output (`|GetArrayItem` (`/Game/Design_Luke/BPC_HP.LimbNames` _bpc_hp) 1))
  ;[0.357 1 0.07456] Left Limb
  (`/Engine/EditorBlueprintResources/StandardMacros.DoOnce` false :!label _label_7
    (:`Completed`
      (if (and (`KismetMathLibrary.ClassIsChildOf` (`GameplayStatics.GetObjectClass` OtherActor) "/Game/Design_Luke/ProjectileChildren/BP_ParentProjectile.BP_ParentProjectile_C") (`BlueprintMapLibrary.Map_Find` (`/Game/Design_Luke/BPC_HP.Active_Limbs` _bpc_hp) _output))
        (message `/Game/Design_Luke/Combat_Interface.Hit_by_Atk` OtherActor 0.0 self _output (`self.BPC_HP`))
        (goto _label_7 :!via `Reset`)
        (else
          (goto _label_7 :!via `Reset`))))))

(event `/Game/Design_Luke/Combat_Interface.DealDamage`
  (params (Dmg :type "Float (double-precision)") (TargetName :type Name) (Source :type "Actor Object Reference") (Widget :type "Widget Object Reference") (Splatterlocation :type "Vector Structure"))
  ;[1 0.151 0.151] Confirm Damage
  (if (not (`self.Invulnerable`))
    (set `self.Invulnerable` true)
    ;;[1 0 0.06264] Apply Damage
    (message `/Game/Design_Luke/Combat_Interface.DealDamage` (`self.BPC_HP`) Dmg TargetName self (`self.HUD_Widget_HP&Stam`) (0.0 0.0 0.0))
    (`KismetSystemLibrary.Delay` 1.73)
    (set `self.Invulnerable` false)))

(event `Key|T`
  (params (Key :type "Key Structure"))
  (:`Pressed`
    (if (`self.LockOn?`)
      (set `self.LockOn?` false)
      (set `self.TargetEnemy(LockedOn)` null)
      (else
        (bind (_closet_enemy _scaned_any_enemy) (`self.GetClosetEnemy` 1500.0))
        (set `self.ClosetEnemy` _closet_enemy)
        (set `self.TargetEnemy(LockedOn)` _closet_enemy)
        (if (< (`self.GetDistanceTo` self (`self.TargetEnemy(LockedOn)`)) 1500.0)
          (if _scaned_any_enemy
            (set `self.LockOn?` true)
            (else
              (set `self.LockOn?` false)))
          (else
            (set `self.TargetEnemy(LockedOn)` null)
            (set `self.LockOn?` false)))))))

(event `CoverCheck`
  (bind _returnvalue (`self.K2_GetActorLocation`))
  (bind _returnvalue_2 (`SceneComponent.K2_GetComponentLocation` (`self.Camera1`)))
  (bind (_outhit _returnvalue_3) (`KismetSystemLibrary.BoxTraceSingle` :`Start` _returnvalue_2 :`End` _returnvalue :`HalfSize` (10.0 50.0 50.0) :`Orientation` (`KismetMathLibrary.FindLookAtRotation` _returnvalue_2 _returnvalue) :`TraceChannel` "TraceTypeQuery1" :`DrawDebugType` "ForDuration"))
  (if _returnvalue_3
    (bind _asstatic_mesh_actor (cast `StaticMeshActor` (`.HitActor` (`GameplayStatics.BreakHitResult` _outhit))))
    (if (not (!= _asstatic_mesh_actor (`self.CoverStaticMeshActor`)))
      (set `self.CoverStaticMeshActor` _asstatic_mesh_actor)
      (bind _staticmeshcomponent (`StaticMeshActor.StaticMeshComponent` _asstatic_mesh_actor))
      (for _index (range (`PrimitiveComponent.GetNumMaterials` _staticmeshcomponent))
        (`KismetArrayLibrary.Array_Add` (`self.CoverStaticMeshActorMaterialList`) (`PrimitiveComponent.GetMaterial` _staticmeshcomponent _index))
        (`PrimitiveComponent.SetMaterial` (`StaticMeshActor.StaticMeshComponent` (`self.CoverStaticMeshActor`)) _index "/Game/Du/Material_Asset/Transparent_Replace.Transparent_Replace")))))

(fn `CycleWeapons`
  (params (Input :type Integer))
  (bind _mesh (`self.Mesh`))
  (bind _value (`BlueprintMapLibrary.Map_Find` (`self.Equipment`) (`self.Selected`)))
  (bind (_returnvalue_location _returnvalue_rotation) (`KismetMathLibrary.BreakTransform` (`SceneComponent.GetSocketTransform` _mesh "Weapon_Sock" "RTS_World")))
  (bind _keys (`BlueprintMapLibrary.Map_Keys` (`self.Equipment`)))
  (bind _selected (`/Game/Design_Luke/BPC_CycleComponent.NextOption` (`self.BPC_CycleComponent`) _keys (`self.Selected`) Input))
  (set `self.Selected` _selected)
  (`self.K2_DestroyActor` (`self.CurrentWeapon`))
  (bind _returnvalue (`|SpawnActorFromClass` _value (`KismetMathLibrary.MakeTransform` _returnvalue_location _returnvalue_rotation (2.0 2.0 2.0)) "Undefined" "MultiplyWithRoot" null null))
  (bind _output_get (set `self.CurrentWeapon` _returnvalue))
  (message `/Game/Design_Luke/Combat_Interface.Set Owner` _output_get _mesh (`self.WeaponArm`) self)
  (`KismetSystemLibrary.PrintString` (`KismetSystemLibrary.GetClassDisplayName` _value)))

(fn `GetClosetEnemy`
  (params (Redius :type "Float (double-precision)"))
  (returns (`Closet Enemy` :type "/Game/Daniel/AI_Types/BP_BaseAI Object Reference") (`Scaned Any Enemy` :type Boolean))
  (bind _returnvalue (`self.K2_GetActorLocation`))
  (bind _enemy (`self.Enemy`))
  (bind (_outhits _returnvalue_2) (`KismetSystemLibrary.SphereTraceMultiForObjects` _returnvalue _returnvalue Redius (`|MakeArray` "ObjectTypeQuery3" :!type "EObjectTypeQuery Enum") false (`|MakeArray` self :!type "Actor Object Reference") "ForDuration"))
  (if _returnvalue_2
    (`KismetArrayLibrary.Array_Clear` (`self.Enemy`))
    (for _array_element _outhits
      (bind _asbp_base_ai (cast `/Game/Daniel/AI_Types/BP_BaseAI` (`.HitActor` (`GameplayStatics.BreakHitResult` _array_element))))
      (`KismetArrayLibrary.Array_AddUnique` (`self.Enemy`) _asbp_base_ai))
    (if (> (`KismetArrayLibrary.Array_Length` _enemy) 0)
      (bind _output_get (set `self.MinDistanceEnemy` (`|GetArrayItem` _enemy)))
      (set `self.MinDistance` (`KismetMathLibrary.Abs` (`self.GetDistanceTo` _output_get self)))
      (for _array_element_2 (`self.Enemy`)
        (if (< (`self.GetDistanceTo` _array_element_2 self) (`self.MinDistance`))
          (set `self.MinDistanceEnemy` _array_element_2)))
      (return (`self.MinDistanceEnemy`) _returnvalue_2))))

(fn `HideBone`
  (params (LostLimb :type Name :default "Elbow_Left"))
  (set `self.Limb_Bone_Name` LostLimb)
  (`SkinnedMeshComponent.HideBoneByName` (`self.Mesh`) (`self.Limb_Bone_Name`) "PBO_None"))

(fn `StartSprinting`
  (set `CharacterMovementComponent.MaxWalkSpeed` 800.0 (`self.CharacterMovement`))
  (set `self.isSprinting` true))

(fn `StopSprinting`
  (set `CharacterMovementComponent.MaxWalkSpeed` 450.0 (`self.CharacterMovement`))
  (set `self.isSprinting` false)
  (`self.StaminaRegen`))

(fn `UnHideBone`
  (params (NewLimb :type Name :default "Elbow_Left"))
  (set `self.Limb_Bone_Name` NewLimb)
  (`SkinnedMeshComponent.UnHideBoneByName` (`self.Mesh`) (`self.Limb_Bone_Name`)))

(fn `UserConstructionScript`
  (set `self.SpawnLocation` (`SceneComponent.K2_GetComponentLocation` (`self.CapsuleComponent`))))