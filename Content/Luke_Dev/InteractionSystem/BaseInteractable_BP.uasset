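; Base interactable pickup actor that places an item in the world for collection into the interacting actor's inventory.
; It loads its ItemInfo from the ItemInfo_DT data table by ItemName, both in the construction script and on BeginPlay.
; On Interact, it passes that info to the instigator's InventoryComponent; a successful pickup shows a popup widget with the item's image and name, then destroys the actor.
; UseItem only prints a debug string.
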(event `self.ReceiveBeginPlay`
  (bind _returnvalue (`|GetDataTableRow` "/Game/Luke_Dev/InteractionSystem/ItemInfo_DT.ItemInfo_DT" (`self.ItemName`))
    (:`then`
      (set `self.ItemInfo` _returnvalue))))

(event `/Game/Luke_Dev/BPI_Interact.Interact`
  (params (Instigator :type "Character Object Reference"))
  (bind ((`ItemName_5_F40122E0455141579E8FC5B354105A3E` _itemname) (`ItemImage_7_66CEC0EC4CA9EA24FB65D987967F7A10` _itemimage)) (break `/Game/Luke_Dev/InteractionSystem/ItemInfo_S` (`self.ItemInfo`)))
  (bind _added (`/Game/Luke_Dev/InteractionSystem/InventoryComponent.PickupItem` (`self.GetComponentByClass` Instigator "/Game/Luke_Dev/InteractionSystem/InventoryComponent.InventoryComponent_C") (`self.ItemInfo`)))
  (if _added
    (bind _returnvalue (`|CreateWidget` "/Game/Design_Luke/Widgets/WB_PickedUp_PopUp.WB_PickedUp_PopUp_C"))
    (`Image.SetBrushFromTexture` (`/Game/Design_Luke/Widgets/WB_PickedUp_PopUp.Item_Image_Icon_32` _returnvalue) _itemimage false)
    (set `TextBlock.Text` _itemname (`/Game/Design_Luke/Widgets/WB_PickedUp_PopUp.TextBlock_112` _returnvalue))
    (`UserWidget.AddToViewport` _returnvalue 0)
    (`self.K2_DestroyActor`)))

(fn `UseItem`
  (`KismetSystemLibrary.PrintString` "ItemUsed"))

(fn `UserConstructionScript`
  (bind _returnvalue (`|GetDataTableRow` "/Game/Luke_Dev/InteractionSystem/ItemInfo_DT.ItemInfo_DT" (`self.ItemName`))
    (:`then`
      (set `self.ItemInfo` _returnvalue))))