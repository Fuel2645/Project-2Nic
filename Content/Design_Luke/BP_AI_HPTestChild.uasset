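; A test AI actor, child of a parent Blueprint, that takes per-limb damage from crossbow bolts through a BPCHP health component.
; Head and left-limb overlaps report hits to the bolt when that limb is active in BPCHP.
; DealDmg, unless invulnerable, sends a stagger message, briefly delays, returns colour-coded feedback to the source, then forwards damage to BPCHP.
; A stagger event grants temporary invulnerability, and Die destroys the actor.
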(event `/Game/Design_Luke/Combat_Interface.Die`
  ;[0 0 0] Die
  (`KismetSystemLibrary.PrintString` "died")
  (`self.K2_DestroyActor`))

(event `/Game/Design_Luke/Combat_Interface.DealDmg`
  (params (Dmg :type Integer) (TargetName :type Name) (Source :type "Actor Object Reference"))
  ;[1 0.151 0.151] Confirm Damage
  (if (not (`self.Invulnerable`))
    (message `/Game/Design_Luke/Combat_Interface.Stagger` self)
    (`KismetSystemLibrary.Delay` 0.15)
    (`KismetSystemLibrary.PrintString` (`KismetStringLibrary.Conv_NameToString` TargetName))
    (`KismetSystemLibrary.PrintString` "hit")
    ;[0 0.7068 1] Feedback
    (bind (_black_dmg _red_dmg _orange_dmg _green_dmg) (`/Game/Design_Luke/BPC_HP.CheckDmgColours` (`self.BPC_HP`)))
    (message `/Game/Design_Luke/Combat_Interface.DmgDealt_Feedback` Source _black_dmg _red_dmg _orange_dmg _green_dmg)
    ;[1 0 0.06264] Apply Damage
    (message `/Game/Design_Luke/Combat_Interface.DealDmg` (`self.BPC_HP`) Dmg TargetName null)))

(event `CustomEvent`
  ;[0.9883 0.5619 1] Stagger
  (set `self.Invulnerable` true)
  (`KismetSystemLibrary.Delay` 0.73)
  (set `self.Invulnerable` false))

(event `self.Box1.OnComponentBeginOverlap`
  (params (OverlappedComponent :type "PrimitiveComponent Object Reference") (OtherActor :type "Actor Object Reference") (OtherComp :type "PrimitiveComponent Object Reference") (OtherBodyIndex :type Integer) (bFromSweep :type Boolean) (SweepResult :type "HitResult Structure (by ref)"))
  (bind _bpc_hp (`self.BPC_HP`))
  (bind _output (`|GetArrayItem` (`/Game/Design_Luke/BPC_HP.LimbNames` _bpc_hp) 2))
  ;[0.357 1 0.07456] Left Limb
  (if (and (== (`GameplayStatics.GetObjectClass` OtherActor) "/Game/Design_Luke/ProjectileChildren/BP_Crossbow_BoltProjectile.BP_Crossbow_BoltProjectile_C") (`BlueprintMapLibrary.Map_Find` (`/Game/Design_Luke/BPC_HP.Active_Limbs` _bpc_hp) _output))
    (message `/Game/Design_Luke/Combat_Interface.Hit_by_Atk` OtherActor 0 self _output (`self.BPC_HP`))))

(event `self.Capsule.OnComponentBeginOverlap`
  (params (OverlappedComponent :type "PrimitiveComponent Object Reference") (OtherActor :type "Actor Object Reference") (OtherComp :type "PrimitiveComponent Object Reference") (OtherBodyIndex :type Integer) (bFromSweep :type Boolean) (SweepResult :type "HitResult Structure (by ref)"))
  (bind _bpc_hp (`self.BPC_HP`))
  (bind _output (`|GetArrayItem` (`/Game/Design_Luke/BPC_HP.LimbNames` _bpc_hp)))
  ;[0.357 1 0.07456] Head
  (if (and (== (`GameplayStatics.GetObjectClass` OtherActor) "/Game/Design_Luke/ProjectileChildren/BP_Crossbow_BoltProjectile.BP_Crossbow_BoltProjectile_C") (`BlueprintMapLibrary.Map_Find` (`/Game/Design_Luke/BPC_HP.Active_Limbs` _bpc_hp) _output))
    (message `/Game/Design_Luke/Combat_Interface.Hit_by_Atk` OtherActor 0 self _output (`self.BPC_HP`))))

(fn `UserConstructionScript`
  (`parent.UserConstructionScript`))