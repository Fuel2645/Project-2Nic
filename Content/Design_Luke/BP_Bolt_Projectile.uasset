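; BP_Bolt_Projectile is a bolt projectile Blueprint that only manages its own lifetime, deferring other startup and construction logic to its parent class.
; On BeginPlay it runs the parent logic, then destroys itself after a few seconds.
; The DmgDealtFeedback event destroys it after a brief delay, presumably once a hit deals damage.
; Its overlap and Tick events are disabled placeholders.
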(event `self.ReceiveBeginPlay`
  (`parent.ReceiveBeginPlay`)
  (`KismetSystemLibrary.Delay` 5.0)
  (`self.K2_DestroyActor`))

(event `/Game/Design_Luke/Combat_Interface.DmgDealt_Feedback`
  (params (Black_Dmg :type Integer) (Red_Dmg :type Integer) (Orange_Dmg :type Integer) (Green_Dmg :type Integer))
  (`KismetSystemLibrary.Delay` 0.12)
  (`self.K2_DestroyActor`))

(fn `UserConstructionScript`
  (`parent.UserConstructionScript`))