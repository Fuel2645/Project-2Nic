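; Rapier weapon hitbox actor, with its attack behavior left unfinished.
; SetOwner stores the owner's skeletal mesh, adds a spring arm to player pawn 0 using the world transform of the Weapon_Grip socket, then snaps the hitbox onto that arm.
; ReleaseAtk only triggers an empty DoOnce, and the chained attack timelines and their lerps are disconnected, so they never run.
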(event `/Game/Design_Luke/Combat_Interface.ReleaseAtk`
  (params (AtkCharge :type Integer))
  (`/Engine/EditorBlueprintResources/StandardMacros.DoOnce` false))

(event `/Game/Design_Luke/Combat_Interface.Set Owner`
  (params (`Owners Skeleton` :type "SkeletalMeshComponent Object Reference") (SrpingArm :type "SpringArmComponent Object Reference"))
  (set `self.Mesh` `Owners Skeleton`)
  (bind _returnvalue (`AddComponent|NODE_AddSpringArmComponent-0` :`self` (`GameplayStatics.GetPlayerPawn` 0) :`RelativeTransform` (`SceneComponent.GetSocketTransform` (`self.Mesh`) "Weapon_Grip" "RTS_World")))
  (bind _output_get (set `self.Srping Arm` _returnvalue))
  (`self.K2_AttachToComponent` _output_get "None" "SnapToTarget" "SnapToTarget" "KeepWorld"))

(fn `UserConstructionScript`
  (`parent.UserConstructionScript`))