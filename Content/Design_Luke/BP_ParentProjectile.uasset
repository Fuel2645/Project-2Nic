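; Base projectile actor that carries damage and shows its strength through the color of a point light.
; HitbyAtk passes damage to targets implementing Combat_Interface, ignoring the actor that spawned it.
; On BeginPlay it messages the player pawn; the ImpactFeedback and DmgDealtFeedback events receive damage thresholds and tint the light black, red, orange or green.
; Overlap and launch events are empty, leaving movement and hit detection outside this graph.
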(event `/Game/Design_Luke/Combat_Interface.Hit_by_Atk`
  (params (Atk_Dmg :type Integer) (HitTarget :type "Actor Object Reference") (TargetName :type Name) (Component_Target :type "ActorComponent Object Reference"))
  (if (!= HitTarget (`self.SpawnedFrom`))
    (if (`KismetSystemLibrary.DoesImplementInterface` HitTarget "/Game/Design_Luke/Combat_Interface.Combat_Interface_C")
      (message `/Game/Design_Luke/Combat_Interface.DealDmg` HitTarget (`self.Damage`) TargetName null))))

(event `self.ReceiveActorBeginOverlap`
  (params (OtherActor :type "Actor Object Reference")))

(event `self.ReceiveBeginPlay`
  ;[1 1 1] Relation to player feedback
  (message `/Game/Design_Luke/Combat_Interface.Impact Feedback` (`GameplayStatics.GetPlayerPawn` 0) self 0 0 0 0))

(event `/Game/Design_Luke/Combat_Interface.Impact Feedback`
  (params (Trigger :type "Actor Object Reference") (Black_Dmg :type Integer) (Red_Dmg :type Integer) (Orange_Dmg :type Integer) (Green_Dmg :type Integer))
  (`|ExecutionSequence`
    (:`then_0`
      (set `self.Black Dmg` Black_Dmg))
    (:`then_1`
      (set `self.Red Dmg` Red_Dmg))
    (:`then_2`
      (set `self.Orange Dmg` Orange_Dmg))
    (:`then_3`
      (set `self.Green Dmg` Green_Dmg))
    (:`then_4`
      (`|ExecutionSequence` :!label _label
        (:`then_0`
          (if (>= (`self.Damage`) (`self.Black Dmg`))
            (`LightComponent.SetLightColor` (`self.PointLight`) (make `LinearColor` 0.1 0.1 0.1 0.5) false)
            (`KismetSystemLibrary.PrintString` "black")))
        (:`then_1`
          (if (== (`self.Damage`) (`self.Red Dmg`))
            (`LightComponent.SetLightColor` (`self.PointLight`) (make `LinearColor` 1.0 0.0 0.0 0.5) true)))
        (:`then_2`
          (if (== (`self.Damage`) (`self.Orange Dmg`))
            (`LightComponent.SetLightColor` (`self.PointLight`) (make `LinearColor` 0.7 0.4 0.4 0.5) true)))
        (:`then_3`
          (if (<= (`self.Damage`) (`self.Green Dmg`))
            (`LightComponent.SetLightColor` (`self.PointLight`) (make `LinearColor` 0.0 1.0 0.0 0.5) true)))))))

(event `/Game/Design_Luke/Combat_Interface.DmgDealt_Feedback`
  (params (Black_Dmg :type Integer) (Red_Dmg :type Integer) (Orange_Dmg :type Integer) (Green_Dmg :type Integer))
  (`|ExecutionSequence`
    (:`then_0`
      (set `self.Black Dmg` Black_Dmg))
    (:`then_1`
      (set `self.Red Dmg` Red_Dmg))
    (:`then_2`
      (set `self.Orange Dmg` Orange_Dmg))
    (:`then_3`
      (set `self.Green Dmg` Green_Dmg))
    (:`then_4`
      (goto _label))))

(event `/Game/Design_Luke/Combat_Interface.Launch Projectile`
  ;[0.4688 0.2995 0.4297] Evidence of alternative but unused launching functionality
)

(fn `UserConstructionScript`)