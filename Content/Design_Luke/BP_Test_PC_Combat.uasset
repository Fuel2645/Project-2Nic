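; Test player character for combat, with a chargeable left-mouse attack and weapon equipping.
; On BeginPlay, if holding a weapon, it spawns the equipped slot's class from the Equipment map and attaches it to the mesh.
; Holding the button raises AttackCharged through a Delay loop.
; Release passes the charge to the weapon, or, without one, fires a crossbow bolt from the R_Grip socket using it as damage.
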(event `Key|LeftMouseButton`
  (params (Key :type "Key Structure"))
  (bind _returnvalue (`self.K2_GetActorRotation`))
  (bind _returnvalue_2 (+ (`SceneComponent.GetSocketLocation` (`self.Mesh`) "R_Grip") (`KismetMathLibrary.GreaterGreater_VectorRotator` (`self.ProjectileOffset`) _returnvalue)))
  (:`Pressed`
    ;[1 1 1] Charge Attack whil
    (bind _output_get (set `self.Charging` true))
    (if _output_get :!label _label
      (`KismetSystemLibrary.Delay` 1.5)
      (`/Engine/EditorBlueprintResources/StandardMacros.IncrementInt` (`self.AttackCharged`)
        (:`  `
          (goto _label)))))
  (:`Released`
    (set `self.Charging` false)
    (if (`self.HoldingWeapon`)
      (message `/Game/Design_Luke/Combat_Interface.ReleaseAtk` (`self.CurrentWeapon`) (`self.AttackCharged`))
      (`KismetSystemLibrary.PrintString` (`KismetStringLibrary.Concat_StrStr` "atk " "dmg = " (`KismetStringLibrary.Conv_IntToString` (`self.AttackCharged`))))
      (set `self.AttackCharged` 1)
      (else
        (set `self.CurrentWeapon` self)
        (`|SpawnActorFromClass` "/Game/Design_Luke/ProjectileChildren/BP_Crossbow_BoltProjectile.BP_Crossbow_BoltProjectile_C" (`KismetMathLibrary.MakeTransform` _returnvalue_2 _returnvalue) "AlwaysSpawn" "OverrideRootScale" null (`self.AttackCharged`) self null)
        (`GameplayStatics.PlaySoundAtLocation` null _returnvalue_2 (struct) 1.0 1.0 0.0 null null null null) ; Play firing sound
      ))))

(event `self.ReceiveBeginPlay`
  (if (`self.HoldingWeapon`)
    (bind _returnvalue (`|SpawnActorFromClass` (`BlueprintMapLibrary.Map_Find` (`self.Equipment`) (`self.SlotEquiped`)) (`SceneComponent.GetSocketTransform` (`self.Mesh`) "None" "RTS_World") "Undefined" "MultiplyWithRoot" null null))
    (set `self.CurrentWeapon` _returnvalue)
    (`self.K2_AttachToComponent` (`self.CurrentWeapon`) (`self.Mesh`) "None" "SnapToTarget" "SnapToTarget" "KeepWorld" true)))

(fn `UserConstructionScript`)