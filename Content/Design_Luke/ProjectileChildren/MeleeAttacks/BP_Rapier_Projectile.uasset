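; Rapier melee attack, built as a projectile child, that performs a thrust with damage set by the attack charge.
; SetOwner snaps it to the owner's spring arm, whose length ReleaseAtk's timelines extend and retract, with capsule overlaps enabled during the thrust behind a DoOnce.
; A separate RunMotion path, apparently test code, lerps the actor from its spawner toward a sent destination, then destroys it.
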(event `/Game/Design_Luke/Combat_Interface.ReleaseAtk`
  (params (AtkCharge :type "Float (double-precision)"))
  (`parent.ReleaseAtk` 0.0)
  (set `self.Damage` AtkCharge)
  (`/Engine/EditorBlueprintResources/StandardMacros.DoOnce` false :!label _label
    (:`Completed`
      (set `PrimitiveComponent.bGenerateOverlapEvents` true (`self.Capsule`))
      (bind (_direction _attack_track) (`Timeline|ReleaseTimeline` :!via `PlayFromStart`)
        (:`Update`
          (set `SpringArmComponent.TargetArmLength` (`KismetMathLibrary.Lerp` 40.0 120.0 _attack_track) (`self.Weapon Arm`)))
        (:`Finished`
          (bind (_direction_2 _attack_track_2) (`Timeline|ReturenTimeline` :!via `PlayFromStart`)
            (:`Update`
              (set `SpringArmComponent.TargetArmLength` (`KismetMathLibrary.Lerp` 120.0 40.0 _attack_track_2) (`self.Weapon Arm`)))
            (:`Finished`
              (set `PrimitiveComponent.bGenerateOverlapEvents` false (`self.Capsule`))
              (set `self.Damage` 1.0)
              (goto _label :!via `Reset`))))))))

(event `/Game/Design_Luke/Combat_Interface.Set Owner`
  (params (`Owners Skeleton` :type "SkeletalMeshComponent Object Reference") (SrpingArm :type "SpringArmComponent Object Reference") (Owner :type "Actor Object Reference"))
  (set `self.Mesh` `Owners Skeleton`)
  (bind _output_get (set `self.Weapon Arm` SrpingArm))
  (`self.K2_AttachToComponent` _output_get "None" "SnapToTarget" "SnapToTarget" "KeepWorld"))

(event `self.ReceiveBeginPlay`
  (`parent.ReceiveBeginPlay`))

(event `self.ReceiveActorBeginOverlap`
  (params (OtherActor :type "Actor Object Reference"))
  (`parent.ReceiveActorBeginOverlap` OtherActor))

(event `/Game/Design_Luke/Combat_Interface.Send_Destination`
  (params (`Sent Destination` :type "Vector Structure") (UpdatedStartLocation :type "Vector Structure") (`Send Rotation` :type "Rotator Structure"))
  ;[0.5052 0.5052 0.5052] Test Evidence
  (set `self.Attack Location` `Sent Destination`)
  (set `self.Starting Location` UpdatedStartLocation)
  (set `self.StartRotation` `Send Rotation`))

(event `/Game/Design_Luke/Combat_Interface.Run_Motion`
  (bind _spawnedfrom (`self.SpawnedFrom`))
  ;[0.5052 0.5052 0.5052] Test Evidence
  (set `self.Starting Location` (`self.K2_GetActorLocation` _spawnedfrom))
  (set `self.StartRotation` (`self.K2_GetActorRotation` _spawnedfrom))
  (bind (_direction _rapier_attack) (`Timeline|Rapier_Attack` :!via `PlayFromStart`)
    (:`Update`
      (message `/Game/Design_Luke/Combat_Interface.Get_Destination` (`self.SpawnedFrom`) self)
      (`self.K2_SetActorLocation` (`KismetMathLibrary.VLerp` (`self.Starting Location`) (`self.Attack Location`) _rapier_attack))
      (`KismetSystemLibrary.PrintString` "update")
      (`self.K2_SetActorRotation` (`self.StartRotation`)))
    (:`Finished`
      (`KismetSystemLibrary.Delay` 0.2)
      (`self.K2_DestroyActor`))))

(fn `UserConstructionScript`
  (`parent.UserConstructionScript`))