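; Base projectile Blueprint for ranged attacks that limits how long each projectile stays in the world.
; BeginPlay runs the parent logic, then destroys the actor after a fixed lifetime of a few seconds.
; The DmgDealtFeedback event destroys it sooner, after a brief delay.
; Construction defers to the parent class, and the overlap and tick events are disabled.
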(event `self.ReceiveBeginPlay`
  (`parent.ReceiveBeginPlay`)
  (`KismetSystemLibrary.Delay` 3.0)
  (`self.K2_DestroyActor`))

(event `/Game/Design_Luke/Combat_Interface.DmgDealt_Feedback`
  (params (Black_Dmg :type "Float (double-precision)") (Red_Dmg :type "Float (double-precision)") (Orange_Dmg :type "Float (double-precision)") (Green_Dmg :type "Float (double-precision)"))
  (`KismetSystemLibrary.Delay` 0.12)
  (`self.K2_DestroyActor`))

(fn `UserConstructionScript`
  (`parent.UserConstructionScript`))