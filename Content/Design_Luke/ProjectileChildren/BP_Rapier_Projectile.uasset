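; Rapier attack projectile child Blueprint that moves by a scripted timeline motion instead of projectile flight.
; BeginPlay deactivates ProjectileMovement and zeroes its speeds.
; RunMotion caches the start location, then the Rapier_Attack timeline lerps the actor up 50 units in Z from that location plus SpawnedFrom's current location, without sweeping.
; The actor destroys itself after a short delay once the timeline finishes.
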(event `self.ReceiveBeginPlay`
  (bind _projectilemovement (`self.ProjectileMovement`))
  (`ActorComponent.Deactivate` (`self.ProjectileMovement`))
  (`parent.ReceiveBeginPlay`)
  (set `ProjectileMovementComponent.InitialSpeed` 0.0 _projectilemovement)
  (set `ProjectileMovementComponent.MaxSpeed` 0.0 _projectilemovement))

(event `/Game/Design_Luke/Combat_Interface.Run_Motion`
  (bind _returnvalue (+ (`self.Starting Location`) (`self.K2_GetActorLocation` (`self.SpawnedFrom`))))
  (set `self.Starting Location` (`self.K2_GetActorLocation`))
  (bind (_direction _rapier_attack) (`Timeline|Rapier_Attack` :!via `PlayFromStart`)
    (:`Update`
      (`self.K2_SetActorLocation` (`KismetMathLibrary.VLerp` _returnvalue (+ _returnvalue (0.0 0.0 50.0)) _rapier_attack)))
    (:`Finished`
      (`KismetSystemLibrary.Delay` 0.2)
      (`self.K2_DestroyActor`))))

(fn `UserConstructionScript`
  (`parent.UserConstructionScript`))