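; BPC_PauseComponent is a component that toggles the pause menu on the IA_Pause input action.
; BeginPlay creates WB_Pause_Menu, adds it to the viewport collapsed and stores a reference.
; Each press flips PauseMenuOpen, switching the menu's visibility, mouse cursor and input mode between game-only and game-and-UI.
; It never pauses the game itself, and prints a "Hello" debug string on each press.
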(event `EnhancedInput|/Game/Design_Luke/Test_Inputs/Individual_InputTest/IA_Pause`
  (params (ActionValue :type "Float (double-precision)") (ElapsedSeconds :type "Float (double-precision)") (TriggeredSeconds :type "Float (double-precision)") (InputAction :type "InputAction Object Reference" :default "/Game/Design_Luke/Test_Inputs/Individual_InputTest/IA_Pause.IA_Pause"))
  (bind _returnvalue (`GameplayStatics.GetPlayerController` 0))
  ;[1 1 1] Show Widget
  (:`Started`
    (`KismetSystemLibrary.PrintString` "Hello")
    (if (`self.PauseMenuOpen`)
      (`Widget.SetVisibility` (`self.PauseMenuRef`) "Collapsed")
      (`WidgetBlueprintLibrary.SetInputMode_GameOnly` _returnvalue)
      (set `PlayerController.bShowMouseCursor` false _returnvalue)
      (set `self.PauseMenuOpen` false)
      (else
        (`Widget.SetVisibility` (`self.PauseMenuRef`) "Visible")
        (set `PlayerController.bShowMouseCursor` true (`GameplayStatics.GetPlayerController` 0))
        (`WidgetBlueprintLibrary.SetInputMode_GameAndUIEx` (`GameplayStatics.GetPlayerController` 0) (`self.PauseMenuRef`) "DoNotLock" false)
        (set `self.PauseMenuOpen` true)))))

(event `self.ReceiveBeginPlay`
  (bind _returnvalue (`|CreateWidget` "/Game/Andy_B1106369/Ui/Pause_Menu/WB_Pause_Menu.WB_Pause_Menu_C"))
  (set `self.PauseMenuRef` _returnvalue)
  (`UserWidget.AddToViewport` _returnvalue 0)
  (`Widget.SetVisibility` (`self.PauseMenuRef`) "Collapsed"))