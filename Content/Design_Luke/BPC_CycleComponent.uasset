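; BPC_CycleComponent is a component with a single helper, NextOption, apparently intended to cycle an index through a list of options.
; NextOption compares CurrentSelection to the Selection length and returns 0 when the length is greater or equal.
; Otherwise it returns the length for a non-positive index, or increments CurrentSelection without assigning that to the returned value.
; The event graph holds only disabled placeholder events.
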(fn `NextOption`
  (params (Selection :type "Array of Integer") (CurrentSelection :type Integer))
  (returns (Selected :type Integer))
  (locals (NewLocalVar :type Integer))
  (if (>= (`KismetArrayLibrary.Array_Length` Selection) CurrentSelection)
    (set `local.NewLocalVar` 0)
    (elif (<= CurrentSelection 0)
      (set `local.NewLocalVar` (`KismetArrayLibrary.Array_Length` Selection))
      (else
        (`/Engine/EditorBlueprintResources/StandardMacros.IncrementInt` CurrentSelection
          (:`  `
            _)))))
  (return (`local.NewLocalVar`)))