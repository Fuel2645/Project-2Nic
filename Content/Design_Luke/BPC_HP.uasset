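; Health component that tracks per-limb hit points and attached state for its owning actor.
; DealDmg subtracts from the named pool, messaging the owner to die on depleted Head or Torso, otherwise to lose that limb.
; Head hits update the passed widget when Source is the player pawn.
; Reattach restores a limb, LimbActiveCheck reports attachment, and CheckDmgColours derives damage-colour thresholds from the highest pool value.
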(event `/Game/Design_Luke/Combat_Interface.DealDmg`
  (params (Dmg :type Integer) (TargetName :type Name) (Source :type "Actor Object Reference") (Widget :type "/Game/Andy_B1106369/Ui/Health_Stamina_Bar/WB_Health_Stamina Object Reference"))
  (bind _health_pools (`self.Health_Pools`))
  (bind _current_target_name (`self.Current Target Name`))
  (bind _current_target_name_2 (`self.Current Target Name`))
  (bind _current_target_name_3 (`self.Current Target Name`))
  (`/Engine/EditorBlueprintResources/StandardMacros.DoOnce` false :!label _label
    (:`Completed`
      (set `self.Current Target Name` TargetName)
      (`|ExecutionSequence`
        (:`then_0`
          (`BlueprintMapLibrary.Map_Add` _health_pools (`self.Current Target Name`) (- (`BlueprintMapLibrary.Map_Find` _health_pools _current_target_name_2) Dmg))
          (if (< (`BlueprintMapLibrary.Map_Find` _health_pools _current_target_name_2) 1)
            (if (or (== _current_target_name_3 "Head") (== _current_target_name_3 "Torso"))
              (message `/Game/Design_Luke/Combat_Interface.Die` (`self.GetOwner`))
              (else
                (message `/Game/Design_Luke/Combat_Interface.LoseLimb` (`self.GetOwner`) (`self.Current Target Name`))
                (`KismetSystemLibrary.PrintString` "lose limb")
                (`BlueprintMapLibrary.Map_Add` (`self.Active_Limbs`) (`self.Current Target Name`))))))
        (:`then_1`
          (if (== Source (`GameplayStatics.GetPlayerPawn` 0))
            (if (== _current_target_name "Head")
              (message `/Game/Andy_B1106369/Ui/Widget_interface.Update Health` Widget (`KismetMathLibrary.Conv_IntToDouble` (`BlueprintMapLibrary.Map_Find` (`self.Health_Pools`) _current_target_name))))))
        (:`then_2`
          (goto _label :!via `Reset`))))))

(event `/Game/Design_Luke/Combat_Interface.Reattach`
  (params (TargetName :type Name))
  (set `self.Current Target Name` TargetName)
  (`BlueprintMapLibrary.Map_Add` (`self.Health_Pools`) (`self.Current Target Name`) 3)
  (`BlueprintMapLibrary.Map_Add` (`self.Active_Limbs`) (`self.Current Target Name`) true))

(fn `CheckDmgColours`
  (returns (Black_Dmg :type Integer) (Red_Dmg :type Integer) (Orange_Dmg :type Integer) (Green_Dmg :type Integer))
  (locals (HighestHealth :type Integer))
  (bind _highesthealth (`local.HighestHealth`))
  (bind _returnvalue (/ _highesthealth 4))
  (bind _values (`BlueprintMapLibrary.Map_Values` (`self.Health_Pools`)))
  (for _array_element _values
    (if (> _array_element (`local.HighestHealth`))
      (set `local.HighestHealth` _array_element)))
  (return _highesthealth (- _highesthealth 1) (+ _returnvalue 1) _returnvalue))

(fn `LimbActiveCheck`
  (params (TargetLimb :type Name))
  (returns (LimbActive :type Boolean))
  (bind (_value _returnvalue) (`BlueprintMapLibrary.Map_Find` (`self.Active_Limbs`) TargetLimb))
  (if _returnvalue
    (if _value
      (return _value)
      (else
        (`KismetSystemLibrary.PrintString` "Limb Removed")
        (return _value)))
    (else
      (`KismetSystemLibrary.PrintString` "No reference to limb found" false true (struct :`R` 1.0 :`B` 0.101925 :`A` 1.0) 5.0) ; Will only come up if given the wrong name or if something that doesn't exist is  been requested.\nCould also be the result of someone remove the limb from the list (the logic wasn't created with things being removed from the index in mind).
    )))