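; Test player character for combat, with diagonal world-axis movement, sprint speed toggling and a dash input that only starts DashCheck.
; BeginPlay adds the test input mapping and, if armed, spawns and attaches the weapon from the Equipment slot.
; Holding attack builds AttackCharged through a delay loop.
; Release sends that charge to CurrentWeapon via message; unarmed, it first targets self and fires a crossbow bolt from the hand socket using charge as damage.
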(event `EnhancedInput|/Game/Design_Luke/Test_Inputs/Individual_InputTest/IA_CombatAtk`
  (params (ActionValue :type Boolean) (ElapsedSeconds :type "Float (double-precision)") (TriggeredSeconds :type "Float (double-precision)") (InputAction :type "InputAction Object Reference" :default "/Game/Design_Luke/Test_Inputs/Individual_InputTest/IA_CombatAtk.IA_CombatAtk"))
  (bind _returnvalue (`self.K2_GetActorRotation`))
  (bind _returnvalue_2 (+ (`SceneComponent.GetSocketLocation` (`self.Mesh`) "R_Grip") (`KismetMathLibrary.GreaterGreater_VectorRotator` (`self.ProjectileOffset`) _returnvalue)))
  (:`Triggered`
    ;[1 1 1] Charge Attack whil
    (bind _output_get (set `self.Charging` true))
    (`KismetSystemLibrary.Delay` 1.5 :!label _label)
    (if _output_get
      (`/Engine/EditorBlueprintResources/StandardMacros.IncrementInt` (`self.AttackCharged`)
        (:`  `
          (goto _label)))))
  (:`Completed`
    (set `self.Charging` false)
    (if (not (`self.HoldingWeapon`))
      (set `self.CurrentWeapon` self)
      (`|SpawnActorFromClass` "/Game/Design_Luke/ProjectileChildren/BP_Crossbow_BoltProjectile.BP_Crossbow_BoltProjectile_C" (`KismetMathLibrary.MakeTransform` _returnvalue_2 _returnvalue) "AlwaysSpawn" "OverrideRootScale" null (`self.AttackCharged`) self null)
      (`GameplayStatics.PlaySoundAtLocation` null _returnvalue_2 (struct) 1.0 1.0 0.0 null null null null) ; Play firing sound
    )
    (message `/Game/Design_Luke/Combat_Interface.ReleaseAtk` (`self.CurrentWeapon`) (`self.AttackCharged`))
    (`KismetSystemLibrary.PrintString` (`KismetStringLibrary.Concat_StrStr` "atk " "dmg = " (`KismetStringLibrary.Conv_IntToString` (`self.AttackCharged`))))
    (set `self.AttackCharged` 1)))

(event `EnhancedInput|/Game/Design_Luke/Test_Inputs/Individual_InputTest/IA_Vertical_LB_Test`
  (params (ActionValue :type "Float (double-precision)") (ElapsedSeconds :type "Float (double-precision)") (TriggeredSeconds :type "Float (double-precision)") (InputAction :type "InputAction Object Reference" :default "/Game/Design_Luke/Test_Inputs/Individual_InputTest/IA_Vertical_LB_Test.IA_Vertical_LB_Test"))
  (:`Triggered`
    (`self.AddMovementInput` (0.5 0.5 0.0) ActionValue)))

(event `Key|LeftMouseButton`
  (params (Key :type "Key Structure")))

(event `self.ReceiveBeginPlay`
  (message `EnhancedInputSubsystemInterface.AddMappingContext` (pcsubsystem `EnhancedInputLocalPlayerSubsystem` (`GameplayStatics.GetPlayerController` 0)) "/Game/Design_Luke/Test_Inputs/D_Luke_Move+Combat_MappingTest.D_Luke_Move+Combat_MappingTest" 0 (struct))
  (if (`self.HoldingWeapon`)
    (bind _returnvalue (`|SpawnActorFromClass` (`BlueprintMapLibrary.Map_Find` (`self.Equipment`) (`self.SlotEquiped`)) (`SceneComponent.GetSocketTransform` (`self.Mesh`) "None" "RTS_World") "Undefined" "MultiplyWithRoot" null null))
    (set `self.CurrentWeapon` _returnvalue)
    (`self.K2_AttachToComponent` (`self.CurrentWeapon`) (`self.Mesh`) "None" "SnapToTarget" "SnapToTarget" "KeepWorld" true)))

(event `EnhancedInput|/Game/Design_Luke/Test_Inputs/Individual_InputTest/IA_Horizontal_LB_Test`
  (params (ActionValue :type "Float (double-precision)") (ElapsedSeconds :type "Float (double-precision)") (TriggeredSeconds :type "Float (double-precision)") (InputAction :type "InputAction Object Reference" :default "/Game/Design_Luke/Test_Inputs/Individual_InputTest/IA_Horizontal_LB_Test.IA_Horizontal_LB_Test"))
  (:`Triggered`
    (`self.AddMovementInput` (-0.5 0.5 0.0) ActionValue)))

(event `EnhancedInput|/Game/Design_Luke/Test_Inputs/Individual_InputTest/IA_Turn`
  (params (ActionValue :type "Vector2D Structure") (ElapsedSeconds :type "Float (double-precision)") (TriggeredSeconds :type "Float (double-precision)") (InputAction :type "InputAction Object Reference" :default "/Game/Design_Luke/Test_Inputs/Individual_InputTest/IA_Turn.IA_Turn")))

(event `EnhancedInput|/Game/Daniel_A/Input/Actions/IA_Dash`
  (params (ActionValue :type Boolean) (ElapsedSeconds :type "Float (double-precision)") (TriggeredSeconds :type "Float (double-precision)") (InputAction :type "InputAction Object Reference" :default "/Game/Daniel_A/Input/Actions/IA_Dash.IA_Dash"))
  (:`Started`
    (`Timeline|DashCheck` :!via `PlayFromStart`)))

(event `EnhancedInput|/Game/Daniel_A/Input/Actions/IA_Sprint`
  (params (ActionValue :type Boolean) (ElapsedSeconds :type "Float (double-precision)") (TriggeredSeconds :type "Float (double-precision)") (InputAction :type "InputAction Object Reference" :default "/Game/Daniel_A/Input/Actions/IA_Sprint.IA_Sprint"))
  ;[0.05098 0.05098 0.05098] Sprinting
  (:`Triggered`
    (`self.StartSprinting`))
  (:`Completed`
    (`self.StopSprinting`)))

(fn `StartSprinting`
  (set `CharacterMovementComponent.MaxWalkSpeed` 600.0 (`self.CharacterMovement`))
  (set `self.isSprinting` true))

(fn `StopSprinting`
  (set `CharacterMovementComponent.MaxWalkSpeed` 300.0 (`self.CharacterMovement`))
  (set `self.isSprinting` false))

(fn `UserConstructionScript`)