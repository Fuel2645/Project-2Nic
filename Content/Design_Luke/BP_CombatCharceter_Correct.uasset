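; Player combat character with per-limb health, charged attacks and stamina-limited sprint and dash.
; Holding left mouse charges damage while a limb is active; release signals the equipped weapon, or spawns a rapier projectile when unarmed.
; Head and arm colliders report crossbow bolt hits; DealDmg forwards damage to BPCHP, triggering stagger invulnerability and colour-tier feedback.
; Lost limbs hide bones; NPC interaction and stamina regen are unwired.
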(event `/Game/Design_Luke/Combat_Interface.LoseLimb`
  (params (LimbName :type Name))
  (`self.HideBone` LimbName :!label _label))

(event `Key|I`
  (params (Key :type "Key Structure"))
  (:`Pressed`
    (goto _label))
  (:`Released`
    (`self.UnHideBone` "None")))

(event `EnhancedInput|/Game/Design_Luke/Test_Inputs/Individual_InputTest/IA_Interact_Main`
  (params (ActionValue :type Boolean) (ElapsedSeconds :type "Float (double-precision)") (TriggeredSeconds :type "Float (double-precision)") (InputAction :type "InputAction Object Reference" :default "/Game/Design_Luke/Test_Inputs/Individual_InputTest/IA_Interact_Main.IA_Interact_Main"))
  ;[1 0.6157 0.826] NPC Interaction
)

(event `self.InteractRadius.OnComponentBeginOverlap`
  (params (OverlappedComponent :type "PrimitiveComponent Object Reference") (OtherActor :type "Actor Object Reference") (OtherComp :type "PrimitiveComponent Object Reference") (OtherBodyIndex :type Integer) (bFromSweep :type Boolean) (SweepResult :type "HitResult Structure (by ref)"))
  ;[1 0.6157 0.826] NPC Interaction
)

(event `self.InteractRadius.OnComponentEndOverlap`
  (params (OverlappedComponent :type "PrimitiveComponent Object Reference") (OtherActor :type "Actor Object Reference") (OtherComp :type "PrimitiveComponent Object Reference") (OtherBodyIndex :type Integer))
  ;[1 0.6157 0.826] NPC Interaction
)

(event `/Game/Luke_Dev/BPI_Interact.ConversationClosed`
  (bind _returnvalue (`GameplayStatics.GetPlayerController` 0))
  ;[1 0.6157 0.826] NPC Interaction
  (set `PlayerController.bShowMouseCursor` false _returnvalue)
  (`WidgetBlueprintLibrary.SetInputMode_GameOnly` _returnvalue))

(event `EnhancedInput|/Game/Design_Luke/Test_Inputs/Individual_InputTest/IA_CombatAtk`
  (params (ActionValue :type Boolean) (ElapsedSeconds :type "Float (double-precision)") (TriggeredSeconds :type "Float (double-precision)") (InputAction :type "InputAction Object Reference" :default "/Game/Design_Luke/Test_Inputs/Individual_InputTest/IA_CombatAtk.IA_CombatAtk")))

(event `Key|LeftMouseButton`
  (params (Key :type "Key Structure"))
  (bind _returnvalue (`self.K2_GetActorRotation`))
  (bind _bpc_hp (`self.BPC_HP`))
  (bind _returnvalue_2 (+ (`SceneComponent.GetSocketLocation` (`self.Mesh`) "R_Grip") (`KismetMathLibrary.GreaterGreater_VectorRotator` (`self.ProjectileOffset`) _returnvalue)))
  (bind _output (`|GetArrayItem` (`/Game/Design_Luke/BPC_HP.LimbNames` _bpc_hp) 3))
  (:`Pressed`
    (if (`/Game/Design_Luke/BPC_HP.LimbActiveCheck` _bpc_hp _output)
      ;[1 1 1] Charge Attack whil
      (bind _output_get (set `self.Charging` true))
      (`KismetSystemLibrary.Delay` 1.4 :!label _label_2)
      (if _output_get
        (`/Engine/EditorBlueprintResources/StandardMacros.IncrementInt` (`self.AttackCharged`)
          (:`  `
            (goto _label_2))))))
  (:`Released`
    (if (`/Game/Design_Luke/BPC_HP.LimbActiveCheck` _bpc_hp _output)
      (set `self.Charging` false)
      (if (not (`self.HoldingWeapon`))
        (set `self.CurrentWeapon` self)
        (`|SpawnActorFromClass` "/Game/Design_Luke/ProjectileChildren/BP_Rapier_Projectile.BP_Rapier_Projectile_C" (`KismetMathLibrary.MakeTransform` _returnvalue_2 _returnvalue) "AlwaysSpawn" "OverrideRootScale" null (`self.AttackCharged`) self null)
        (`GameplayStatics.PlaySoundAtLocation` null _returnvalue_2 (struct) 1.0 1.0 0.0 null null null null) ; Play firing sound
      )
      (message `/Game/Design_Luke/Combat_Interface.ReleaseAtk` (`self.CurrentWeapon`) (`self.AttackCharged`))
      (`KismetSystemLibrary.PrintString` (`KismetStringLibrary.Concat_StrStr` "atk " "dmg = " (`KismetStringLibrary.Conv_IntToString` (`self.AttackCharged`))))
      (set `self.AttackCharged` 1))))

(event `EnhancedInput|/Game/Design_Luke/Test_Inputs/Individual_InputTest/IA_Vertical_LB_Test`
  (params (ActionValue :type "Float (double-precision)") (ElapsedSeconds :type "Float (double-precision)") (TriggeredSeconds :type "Float (double-precision)") (InputAction :type "InputAction Object Reference" :default "/Game/Design_Luke/Test_Inputs/Individual_InputTest/IA_Vertical_LB_Test.IA_Vertical_LB_Test"))
  (:`Triggered`
    (`self.AddMovementInput` (-0.5 0.5 0.0) ActionValue)))

(event `self.ReceiveBeginPlay`
  (message `EnhancedInputSubsystemInterface.AddMappingContext` (pcsubsystem `EnhancedInputLocalPlayerSubsystem` (`GameplayStatics.GetPlayerController` 0)) "/Game/Design_Luke/Test_Inputs/D_Luke_Move+Combat_MappingTest.D_Luke_Move+Combat_MappingTest" 0 (struct))
  (if (`self.HoldingWeapon`)
    (bind _returnvalue (`|SpawnActorFromClass` (`BlueprintMapLibrary.Map_Find` (`self.Equipment`) (`self.SlotEquiped`)) (`SceneComponent.GetSocketTransform` (`self.Mesh`) "None" "RTS_World") "Undefined" "MultiplyWithRoot" null null))
    (set `self.CurrentWeapon` _returnvalue)
    (`self.K2_AttachToComponent` (`self.CurrentWeapon`) (`self.Mesh`) "None" "SnapToTarget" "SnapToTarget" "KeepWorld" true)))

(event `EnhancedInput|/Game/Design_Luke/Test_Inputs/Individual_InputTest/IA_Horizontal_LB_Test`
  (params (ActionValue :type "Float (double-precision)") (ElapsedSeconds :type "Float (double-precision)") (TriggeredSeconds :type "Float (double-precision)") (InputAction :type "InputAction Object Reference" :default "/Game/Design_Luke/Test_Inputs/Individual_InputTest/IA_Horizontal_LB_Test.IA_Horizontal_LB_Test"))
  (:`Triggered`
    (`self.AddMovementInput` (-0.5 -0.5 0.0) ActionValue)))

(event `EnhancedInput|/Game/Design_Luke/Test_Inputs/Individual_InputTest/IA_Turn`
  (params (ActionValue :type "Vector2D Structure") (ElapsedSeconds :type "Float (double-precision)") (TriggeredSeconds :type "Float (double-precision)") (InputAction :type "InputAction Object Reference" :default "/Game/Design_Luke/Test_Inputs/Individual_InputTest/IA_Turn.IA_Turn"))
  ;[1 1 1] evidence for learning
)

(event `/Game/Design_Luke/Combat_Interface.Impact Feedback`
  (params (Trigger :type "Actor Object Reference") (Black_Dmg :type Integer) (Red_Dmg :type Integer) (Orange_Dmg :type Integer) (Green_Dmg :type Integer))
  ;[1 1 1] Spawned Projectiles Feedback
  (bind (_black_dmg _red_dmg _orange_dmg _green_dmg) (`/Game/Design_Luke/BPC_HP.CheckDmgColours` (`self.BPC_HP`)))
  (message `/Game/Design_Luke/Combat_Interface.Impact Feedback` Trigger null _black_dmg _red_dmg _orange_dmg _green_dmg))

(event `EnhancedInput|/Game/Daniel_A/Input/Actions/IA_Sprint`
  (params (ActionValue :type Boolean) (ElapsedSeconds :type "Float (double-precision)") (TriggeredSeconds :type "Float (double-precision)") (InputAction :type "InputAction Object Reference" :default "/Game/Daniel_A/Input/Actions/IA_Sprint.IA_Sprint"))
  ;[0.05098 0.05098 0.05098] Sprinting
  (:`Triggered`
    (`self.StartSprinting`))
  (:`Completed`
    (`self.StopSprinting`)))

(event `EnhancedInput|/Game/Daniel_A/Input/Actions/IA_Dash`
  (params (ActionValue :type Boolean) (ElapsedSeconds :type "Float (double-precision)") (TriggeredSeconds :type "Float (double-precision)") (InputAction :type "InputAction Object Reference" :default "/Game/Daniel_A/Input/Actions/IA_Dash.IA_Dash"))
  (bind (_velocity_x _velocity_y _velocity_z) (`KismetMathLibrary.BreakVector` (`MovementComponent.Velocity` (`self.CharacterMovement`))))
  ;[1 1 1] Dash/Sprint
  (:`Started`
    (bind (_direction _distance) (`Timeline|Timeline` :!via `PlayFromStart`)
      (:`Update`
        (bind (_returnvalue_x _returnvalue_y) (`KismetMathLibrary.BreakVector` (* (`self.GetActorForwardVector`) (* _distance (`self.Dash Distance`)))))
        (set `MovementComponent.Velocity` (`KismetMathLibrary.MakeVector` _returnvalue_x _returnvalue_y _velocity_z) (`self.CharacterMovement`))
        (if (`|GetInputActionValue`)
          (`self.StartSprinting`)))
      (:`Finished`
        (set `self.Stamina` (`KismetMathLibrary.Clamp` (- (`self.Stamina`) 20) 0 (`self.Max Stamina`)))
        (`KismetSystemLibrary.PrintString` (`KismetStringLibrary.Conv_IntToString` (`self.Stamina`))))))
  (:`Completed`
    (`self.StopSprinting`)))

(event `StamDrain`
  (bind _output_get (set `self.Stamina` (`KismetMathLibrary.Clamp` (- (`self.Stamina`) 1) 0 (`self.Max Stamina`))))
  (if (== _output_get 0)
    (`self.StopSprinting`)
    (elif (`self.isSprinting`)
      (`KismetSystemLibrary.Delay` 0.2)
      (`self.StamDrain`)
      (`KismetSystemLibrary.PrintString` (`KismetStringLibrary.Conv_IntToString` (`self.Stamina`))))))

(event `StaminaRegen`
  (bind _output_get (set `self.Stamina` (`KismetMathLibrary.Clamp` (+ (`self.Stamina`) 5) 0 (`self.Max Stamina`))))
  (if (== _output_get (`self.Max Stamina`))
    _
    (elif (not (`self.isSprinting`))
      (`KismetSystemLibrary.Delay` 2.0)
      (`self.StaminaRegen`)
      (`KismetSystemLibrary.PrintString` (`KismetStringLibrary.Conv_IntToString` (`self.Stamina`))))))

(event `/Game/Design_Luke/Combat_Interface.Die`
  ;[0 0 0] Die
  (`KismetSystemLibrary.PrintString` "died")
  (`self.K2_DestroyActor`))

(event `/Game/Design_Luke/Combat_Interface.DealDmg`
  (params (Dmg :type Integer) (TargetName :type Name) (Source :type "Actor Object Reference"))
  ;[1 0.151 0.151] Confirm Damage
  (`/Engine/EditorBlueprintResources/StandardMacros.DoOnce` false :!label _label_3
    (:`Completed`
      (`|ExecutionSequence`
        (:`then_0`
          (if (`self.Invulnerable`)
            (goto _label_3 :!via `Reset`)
            (else
              (message `/Game/Design_Luke/Combat_Interface.Stagger` self)
              (`KismetSystemLibrary.Delay` 0.15)
              (`KismetSystemLibrary.PrintString` (`KismetStringLibrary.Conv_NameToString` TargetName))
              (`KismetSystemLibrary.PrintString` "hit")
              ;[0 0.7068 1] Feedback
              (bind (_black_dmg _red_dmg _orange_dmg _green_dmg) (`/Game/Design_Luke/BPC_HP.CheckDmgColours` (`self.BPC_HP`)))
              (message `/Game/Design_Luke/Combat_Interface.DmgDealt_Feedback` Source _black_dmg _red_dmg _orange_dmg _green_dmg)
              ;[1 0 0.06264] Apply Damage
              (message `/Game/Design_Luke/Combat_Interface.DealDmg` (`self.BPC_HP`) Dmg TargetName null))))
        (:`then_1`
          (goto _label_3 :!via `Reset`))))))

(event `/Game/Design_Luke/Combat_Interface.Stagger`
  ;[0.9883 0.5619 1] Stagger
  (`/Engine/EditorBlueprintResources/StandardMacros.DoOnce` false :!label _label_4
    (:`Completed`
      (set `self.Invulnerable` true)
      (`KismetSystemLibrary.Delay` 0.73)
      (set `self.Invulnerable` false)
      (goto _label_4 :!via `Reset`))))

(event `self.L_Arm_Box.OnComponentBeginOverlap`
  (params (OverlappedComponent :type "PrimitiveComponent Object Reference") (OtherActor :type "Actor Object Reference") (OtherComp :type "PrimitiveComponent Object Reference") (OtherBodyIndex :type Integer) (bFromSweep :type Boolean) (SweepResult :type "HitResult Structure (by ref)"))
  (bind _bpc_hp (`self.BPC_HP`))
  (bind _output (`|GetArrayItem` (`/Game/Design_Luke/BPC_HP.LimbNames` _bpc_hp) 2))
  ;[0.357 1 0.07456] Left Limb
  (`/Engine/EditorBlueprintResources/StandardMacros.DoOnce` false :!label _label_5
    (:`Completed`
      (`|ExecutionSequence`
        (:`then_0`
          (if (and (== (`GameplayStatics.GetObjectClass` OtherActor) "/Game/Design_Luke/ProjectileChildren/BP_Crossbow_BoltProjectile.BP_Crossbow_BoltProjectile_C") (`BlueprintMapLibrary.Map_Find` (`/Game/Design_Luke/BPC_HP.Active_Limbs` _bpc_hp) _output))
            (message `/Game/Design_Luke/Combat_Interface.Hit_by_Atk` OtherActor 0 self _output (`self.BPC_HP`))))
        (:`then_1`
          (goto _label_5 :!via `Reset`))))))

(event `self.Head_Sphere.OnComponentBeginOverlap`
  (params (OverlappedComponent :type "PrimitiveComponent Object Reference") (OtherActor :type "Actor Object Reference") (OtherComp :type "PrimitiveComponent Object Reference") (OtherBodyIndex :type Integer) (bFromSweep :type Boolean) (SweepResult :type "HitResult Structure (by ref)"))
  (bind _bpc_hp (`self.BPC_HP`))
  (bind _output (`|GetArrayItem` (`/Game/Design_Luke/BPC_HP.LimbNames` _bpc_hp)))
  ;[0.357 1 0.07456] Head
  (`/Engine/EditorBlueprintResources/StandardMacros.DoOnce` false :!label _label_6
    (:`Completed`
      (`|ExecutionSequence`
        (:`then_0`
          (if (and (== (`GameplayStatics.GetObjectClass` OtherActor) "/Game/Design_Luke/ProjectileChildren/BP_Crossbow_BoltProjectile.BP_Crossbow_BoltProjectile_C") (`BlueprintMapLibrary.Map_Find` (`/Game/Design_Luke/BPC_HP.Active_Limbs` _bpc_hp) _output))
            (message `/Game/Design_Luke/Combat_Interface.Hit_by_Atk` OtherActor 0 self _output (`self.BPC_HP`))))
        (:`then_1`
          (goto _label_6 :!via `Reset`))))))

(event `self.R_Arm_Box.OnComponentBeginOverlap`
  (params (OverlappedComponent :type "PrimitiveComponent Object Reference") (OtherActor :type "Actor Object Reference") (OtherComp :type "PrimitiveComponent Object Reference") (OtherBodyIndex :type Integer) (bFromSweep :type Boolean) (SweepResult :type "HitResult Structure (by ref)"))
  (bind _bpc_hp (`self.BPC_HP`))
  (bind _output (`|GetArrayItem` (`/Game/Design_Luke/BPC_HP.LimbNames` _bpc_hp) 3))
  ;[0.357 1 0.07456] Right Limb
  (`/Engine/EditorBlueprintResources/StandardMacros.DoOnce` false :!label _label_7
    (:`Completed`
      (`|ExecutionSequence`
        (:`then_0`
          (if (and (== (`GameplayStatics.GetObjectClass` OtherActor) "/Game/Design_Luke/ProjectileChildren/BP_Crossbow_BoltProjectile.BP_Crossbow_BoltProjectile_C") (`BlueprintMapLibrary.Map_Find` (`/Game/Design_Luke/BPC_HP.Active_Limbs` _bpc_hp) _output))
            (message `/Game/Design_Luke/Combat_Interface.Hit_by_Atk` OtherActor 0 self _output (`self.BPC_HP`))))
        (:`then_1`
          (goto _label_7 :!via `Reset`))))))

(fn `CheckDmgColours`
  (returns (Black_Dmg :type Integer) (Red_Dmg :type Integer) (Orange_Dmg :type Integer) (Green_Dmg :type Integer))
  (locals (HighestHealth :type Integer))
  (bind _highesthealth (`local.HighestHealth`))
  (bind _values (`BlueprintMapLibrary.Map_Values` (`/Game/Design_Luke/BPC_HP.Health_Pools` (`self.BPC_HP`))))
  (for _array_element _values
    (if (> _array_element (`local.HighestHealth`))
      (set `local.HighestHealth` _array_element)))
  (return _highesthealth (- _highesthealth 1) (/ _highesthealth 2) (/ _highesthealth 4)))

(fn `HideBone`
  (params (LostLimb :type Name))
  (locals (Limb_Bone_Name :type Name))
  (bind _mesh (`self.Mesh`))
  (set `local.Limb_Bone_Name` LostLimb)
  (`SkinnedMeshComponent.HideBoneByName` _mesh (`local.Limb_Bone_Name`) "PBO_None")
  (`PrimitiveComponent.PutRigidBodyToSleep` _mesh "Elbow_Left"))

(fn `StartSprinting`
  (set `CharacterMovementComponent.MaxWalkSpeed` 800.0 (`self.CharacterMovement`))
  (set `self.isSprinting` true)
  (`self.StamDrain`))

(fn `StopSprinting`
  (set `CharacterMovementComponent.MaxWalkSpeed` 450.0 (`self.CharacterMovement`))
  (set `self.isSprinting` false))

(fn `UnHideBone`
  (params (NewLimb :type Name))
  (`SkinnedMeshComponent.UnHideBoneByName` (`self.Mesh`) "Elbow_Left"))

(fn `UserConstructionScript`)