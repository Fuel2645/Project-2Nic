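; Trap actor that endlessly fires arrows or flames, chosen by the FlameTrap flag, from six ShootingDirection components.
; The construction script caps NumberOfTraps at six, builds cumulative Distance offsets and shifts the later emitters along world Y.
; After a short delay at BeginPlay, Firing spawns a projectile at each emitter via a delayed loop, then calls itself again.
; Firing always uses all six emitters, regardless of NumberOfTraps.
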(event `self.ReceiveBeginPlay`
  (`KismetSystemLibrary.Delay` 1.0)
  (`self.Firing`))

(event `Firing`
  (bind _array_element (`/Game/Patryk_Klich/MacroLibrary.ForEach Loop with Delay` (`|MakeArray` (`SceneComponent.K2_GetComponentToWorld` (`self.Shooting Direction0`)) (`SceneComponent.K2_GetComponentToWorld` (`self.Shooting Direction1`)) (`SceneComponent.K2_GetComponentToWorld` (`self.Shooting Direction2`)) (`SceneComponent.K2_GetComponentToWorld` (`self.Shooting Direction3`)) (`SceneComponent.K2_GetComponentToWorld` (`self.Shooting Direction4`)) (`SceneComponent.K2_GetComponentToWorld` (`self.Shooting Direction5`))) 1.0)
    (:`LoopBody`
      (`|SpawnActorFromClass` (`self.ProjectileType`) (`KismetMathLibrary.MakeTransform` (.location _array_element) (`KismetMathLibrary.MakeRotator` 0.0 (.pitch (.rotation _array_element)) (.yaw (.rotation _array_element))) (.scale _array_element)) "Undefined" "MultiplyWithRoot" null null))
    (:`Completed`
      (`self.Firing`))))

(fn `AddTrapsToArray`
  (if (> (`self.NumberOfTraps`) 6)
    (set `self.NumberOfTraps` 6))
  (for _ (range 1 (+ (`self.NumberOfTraps`) 1))
    (`KismetArrayLibrary.Array_Add` (`self.NumberOfTrapsArray`))))

(fn `DistanceCalculation`
  (bind _numberoftrapsarray (`self.NumberOfTrapsArray`))
  (for (_array_element _array_index) _numberoftrapsarray
    (if (!= _array_index 0)
      (`KismetArrayLibrary.Array_Set` _numberoftrapsarray _array_index (+ (`KismetMathLibrary.MakeVector` 0.0 (`.Y` (`KismetMathLibrary.BreakVector3f` _array_element))) (`KismetMathLibrary.MakeVector` 0.0 (`self.CalculationDistance`))))
      (set `self.CalculationDistance` (+ (`self.Distance`) (`self.CalculationDistance`))))))

(fn `DistanceDisplay`
  (bind _shooting_direction2 (`self.Shooting Direction2`))
  (bind _shooting_direction3 (`self.Shooting Direction3`))
  (bind _shooting_direction4 (`self.Shooting Direction4`))
  (bind _shooting_direction5 (`self.Shooting Direction5`))
  (bind _shooting_direction1 (`self.Shooting Direction1`))
  (for (_array_element _array_index) (`self.NumberOfTrapsArray`)
    (switch `int` _array_index
      (:`1`
        (`SceneComponent.K2_SetWorldLocation` _shooting_direction1 (+ _array_element (`SceneComponent.K2_GetComponentLocation` _shooting_direction1)) false false))
      (:`2`
        (`SceneComponent.K2_SetWorldLocation` _shooting_direction2 (+ _array_element (`SceneComponent.K2_GetComponentLocation` _shooting_direction2)) false false))
      (:`3`
        (`SceneComponent.K2_SetWorldLocation` _shooting_direction3 (+ _array_element (`SceneComponent.K2_GetComponentLocation` _shooting_direction3)) false false))
      (:`4`
        (`SceneComponent.K2_SetWorldLocation` _shooting_direction4 (+ _array_element (`SceneComponent.K2_GetComponentLocation` _shooting_direction4)) false false))
      (:`5`
        (`SceneComponent.K2_SetWorldLocation` _shooting_direction5 (+ _array_element (`SceneComponent.K2_GetComponentLocation` _shooting_direction5)) false false)))))

(fn `FlameTrapCheck`
  (if (`self.FlameTrap`)
    (set `self.ProjectileType` "/Game/Patryk_Klich/projectiles/BP_flame.BP_flame_C")
    (else
      (set `self.ProjectileType` "/Game/Patryk_Klich/projectiles/BP_Arrow.BP_Arrow_C"))))

(fn `UserConstructionScript`
  (`|ExecutionSequence`
    (:`then_0`
      (`self.AddTrapsToArray`))
    (:`then_1`
      (`self.FlameTrapCheck`))
    (:`then_2`
      (set `self.CalculationDistance` (`self.Distance`)))
    (:`then_3`
      (`self.DistanceCalculation`))
    (:`then_4`
      (`self.DistanceDisplay`))))