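; BP_SpikeTrap is a spike pit trap hidden under a cracked floor, lethal to the player character.
; Entering the floor's trigger box prints a debug string, then destroys the cracked floor after a short delay.
; Overlapping the kill box destroys the player character outright.
; The construction script sizes the trap from SpikeSize by destroying spike meshes: Medium drops the outer ring, Small also drops the middle ring.
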(event `self.ReceiveBeginPlay`)

(event `self.CrackedFloorTriggerBox.OnComponentBeginOverlap`
  (params (OverlappedComponent :type "PrimitiveComponent Object Reference") (OtherActor :type "Actor Object Reference") (OtherComp :type "PrimitiveComponent Object Reference") (OtherBodyIndex :type Integer) (bFromSweep :type Boolean) (SweepResult :type "HitResult Structure (by ref)"))
  (if (== OtherActor (`GameplayStatics.GetPlayerCharacter` 0))
    (`KismetSystemLibrary.PrintString` "FloorCracking")
    (`KismetSystemLibrary.Delay` 1.0)
    (`ActorComponent.K2_DestroyComponent` (`self.CrackedFloor`))))

(event `self.KillBox.OnComponentBeginOverlap`
  (params (OverlappedComponent :type "PrimitiveComponent Object Reference") (OtherActor :type "Actor Object Reference") (OtherComp :type "PrimitiveComponent Object Reference") (OtherBodyIndex :type Integer) (bFromSweep :type Boolean) (SweepResult :type "HitResult Structure (by ref)"))
  (if (== OtherActor (`GameplayStatics.GetPlayerCharacter` 0))
    (`self.K2_DestroyActor` OtherActor)))

(fn `UserConstructionScript`
  (switch `/Game/Patryk_Klich/SpikeEnum` (`self.SpikeSize`)
    (:`NewEnumerator0`
      (for _array_element (`|MakeArray` (`self.MiddleRing`) (`self.StaticMesh12`) (`self.StaticMesh13`) (`self.StaticMesh8`) (`self.StaticMesh2`) (`self.StaticMesh3`) (`self.StaticMesh6`) (`self.StaticMesh11`))
        (`ActorComponent.K2_DestroyComponent` _array_element)))
    (:`NewEnumerator1`
      _))
  (for _array_element_2 (`|MakeArray` (`self.OuterRing`) (`self.StaticMesh4`) (`self.StaticMesh`) (`self.StaticMesh16`) (`self.StaticMesh17`) (`self.StaticMesh18`) (`self.StaticMesh19`) (`self.StaticMesh5`) (`self.StaticMesh9`) (`self.5`) (`self.4`) (`self.3`) (`self.2`) (`self.StaticMesh15`) (`self.StaticMesh14`) (`self.StaticMesh10`))
    (`ActorComponent.K2_DestroyComponent` _array_element_2)))