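; Puzzle floor tile in a four-step sequence that triggers DoorToOpen's lever action when the tiles are stepped on in order.
; A correct overlap lights the tile and passes progress to the next Order tile in TIlesArray.
; A wrong step resets every tile and flashes them red twice.
; ShowPattern previews the sequence with Order-based delayed blinks, and the last tile then restores previously lit tiles.
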(event `ShowPattern`
  (bind _cube (`self.Cube`))
  (bind _cube_2 (`self.Cube`))
  ;[1 1 1] ShowingCorrectPattern
  (if (not (`self.ShowingPattern`))
    (set `self.ShowingPattern` true)
    (if (`self.Check if lit up`)
      (set `self.WasLit` true)
      (else
        (set `self.WasLit` false)))
    (`PrimitiveComponent.SetMaterial` (`self.Cube`) 0 "/Engine/BasicShapes/BasicShapeMaterial.BasicShapeMaterial")
    (switch `int` (`self.Order`)
      (:`0`
        (`KismetSystemLibrary.Delay` 0.5)
        (if (`self.WasLit`) :!label _label
          (`PrimitiveComponent.SetMaterial` _cube_2 0 (`self.LightUpMaterial`))
          (`KismetSystemLibrary.Delay` 0.5)
          (`PrimitiveComponent.SetMaterial` _cube_2 0 "/Engine/BasicShapes/BasicShapeMaterial.BasicShapeMaterial")
          (else
            (`PrimitiveComponent.SetMaterial` _cube 0 (`self.LightUpMaterial`))
            (`KismetSystemLibrary.Delay` 0.5)
            (`PrimitiveComponent.SetMaterial` _cube 0 "/Engine/BasicShapes/BasicShapeMaterial.BasicShapeMaterial"))))
      (:`1`
        (`KismetSystemLibrary.Delay` 1.0)
        (goto _label))
      (:`2`
        (`KismetSystemLibrary.Delay` 1.5)
        (goto _label))
      (:`3`
        (`KismetSystemLibrary.Delay` 2.0)
        (`|ExecutionSequence`
          (:`then_0`
            (goto _label))
          (:`then_1`
            (`KismetSystemLibrary.Delay` 0.5)
            (`self.BringBackColours`)))))))

(event `self.Box.OnComponentBeginOverlap`
  (params (OverlappedComponent :type "PrimitiveComponent Object Reference") (OtherActor :type "Actor Object Reference") (OtherComp :type "PrimitiveComponent Object Reference") (OtherBodyIndex :type Integer) (bFromSweep :type Boolean) (SweepResult :type "HitResult Structure (by ref)"))
  (bind _tilesarray (`self.TIlesArray`))
  (if (== (`self.CurrentOrder`) (`self.Order`))
    (`PrimitiveComponent.SetMaterial` (`self.Cube`) 0 (`self.LightUpMaterial`))
    (if (== (`self.Order`) 3)
      (`/Engine/EditorBlueprintResources/StandardMacros.DoOnce` false
        (:`Completed`
          (`/Game/Luke_Dev/Door/Door.LeverAction` (`self.DoorToOpen`))))
      (else
        (for _array_element (`self.TIlesArray`)
          (if (== (`/Game/Patryk_Klich/puzzles/BP_PuzzleTile.Order` _array_element) (+ (`self.Order`) 1))
            (message `/Game/Patryk_Klich/puzzles/BPI_Puzzles.OrderAddition` _array_element (`self.CurrentOrder`))))))
    (else
      (for _array_element_2 _tilesarray
        (set `/Game/Patryk_Klich/puzzles/BP_PuzzleTile.CurrentOrder` 0 _array_element_2)
        (`PrimitiveComponent.SetMaterial` (`/Game/Patryk_Klich/puzzles/BP_PuzzleTile.Cube` _array_element_2) 0 "/Engine/BasicShapes/BasicShapeMaterial.BasicShapeMaterial"))
      (`self.Flashing` _tilesarray _tilesarray _tilesarray _tilesarray))))

(event `/Game/Patryk_Klich/puzzles/BPI_Puzzles.OrderAddition`
  (params (NewParam :type Integer))
  (bind _result (`/Engine/EditorBlueprintResources/StandardMacros.IncrementInt` NewParam)
    (:`  `
      (set `self.CurrentOrder` _result))))

(fn `BringBackColours`
  (for _array_element (`self.TIlesArray`)
    (if (`/Game/Patryk_Klich/puzzles/BP_PuzzleTile.WasLit` _array_element)
      (`PrimitiveComponent.SetMaterial` (`/Game/Patryk_Klich/puzzles/BP_PuzzleTile.Cube` _array_element) 0 (`self.LightUpMaterial`)))
    (set `/Game/Patryk_Klich/puzzles/BP_PuzzleTile.ShowingPattern` false _array_element)))

(fn `UserConstructionScript`
  (if (== (`self.Order`) 3)
    _))