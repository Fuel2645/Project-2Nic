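; Cog puzzle actor that turns a quarter step on Interact and passes the turn along linked left and right neighbor cogs.
; A timeline lerps the pitch clockwise or counterclockwise, then steps the four-way CogState enum and prints a debug message if it matches CorrectState.
; The construction script highlights the sphere matching CogState and caches the starting rotation.
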(event `CorrectPositionCheck`
  (if (`|EnumEquality` (`self.CorrectState`) (`self.cogState`))
    (`KismetSystemLibrary.PrintString` "Correct Place")))

(event `/Game/Patryk_Klich/puzzles/BPI_Puzzles.CogConnectionLeft`
  (bind _cogtotheleft (`self.CogToTheLeft`))
  (bind (_gear_rotation_roll _gear_rotation_pitch _gear_rotation_yaw) (`KismetMathLibrary.BreakRotator` (`self.Gear Rotation`)))
  (bind (_gear_rotation_roll_2 _gear_rotation_pitch_2 _gear_rotation_yaw_2) (`KismetMathLibrary.BreakRotator` (`self.Gear Rotation`)))
  (`/Engine/EditorBlueprintResources/StandardMacros.IsValid` _cogtotheleft :!label _label
    (:`Is Valid`
      (`/Game/Patryk_Klich/puzzles/BPI_Puzzles.CogConnectionLeft` _cogtotheleft))
    (:`Is Not Valid`
      _))
  (if (`self.CounterClockwise`) :!label _label_2
    (set `self.Angle` 90.0)
    (else
      (set `self.Angle` -90.0)))
  (set `self.GearEnd Rotation` (`KismetMathLibrary.MakeRotator` _gear_rotation_roll_2 (+ _gear_rotation_pitch_2 (`self.Angle`)) _gear_rotation_yaw_2))
  (bind (_direction _newtrack_0) (`Timeline|rotation` :!via `PlayFromStart`)
    (:`Update`
      (`self.K2_SetActorRotation` (`KismetMathLibrary.RLerp` (`self.Gear Rotation`) (`self.GearEnd Rotation`) _newtrack_0)))
    (:`Finished`
      (set `self.Gear Rotation` (`KismetMathLibrary.MakeRotator` _gear_rotation_roll (+ _gear_rotation_pitch (`self.Angle`)) _gear_rotation_yaw))
      (if (`self.CounterClockwise`)
        (`self.Current Cog State`)
        (else
          (`self.Current Cog State ClockWise`)))
      (`self.CorrectPositionCheck`))))

(event `/Game/Luke_Dev/BPI_Interact.Interact`
  (bind _cogtotheright (`self.CogToTheRight`))
  (`|ExecutionSequence`
    (:`then_0`
      (goto _label))
    (:`then_1`
      (`/Engine/EditorBlueprintResources/StandardMacros.IsValid` _cogtotheright :!label _label_3
        (:`Is Valid`
          (`/Game/Patryk_Klich/puzzles/BPI_Puzzles.CogConnectionRight` _cogtotheright)
          (goto _label_2))
        (:`Is Not Valid`
          (goto _label_2))))))

(event `/Game/Patryk_Klich/puzzles/BPI_Puzzles.CogConnectionRight`
  (goto _label_3))

(fn `adjustRotation`
  (bind _array (`|MakeArray` (`self.SphereUP`) (`self.SphereRIGHT`) (`self.SphereDOWN`) (`self.SphereLEFT`)))
  (switch `/Game/Patryk_Klich/CogEnum` (`self.cogState`)
    (:`NewEnumerator0`
      (for (_array_element _array_index) _array
        (if (== _array_index 0)
          (`PrimitiveComponent.SetMaterial` _array_element 0 "/Engine/VREditor/BasicMeshes/MI_Cube_03.MI_Cube_03")
          (else
            (`PrimitiveComponent.SetMaterial` _array_element 0 "/Engine/BasicShapes/BasicShapeMaterial.BasicShapeMaterial")))))
    (:`NewEnumerator1`
      (for (_array_element_2 _array_index_2) _array
        (if (== _array_index_2 1)
          (`PrimitiveComponent.SetMaterial` _array_element_2 0 "/Engine/VREditor/BasicMeshes/MI_Cube_03.MI_Cube_03")
          (else
            (`PrimitiveComponent.SetMaterial` _array_element_2 0 "/Engine/BasicShapes/BasicShapeMaterial.BasicShapeMaterial")))))
    (:`NewEnumerator2`
      (for (_array_element_3 _array_index_3) _array
        (if (== _array_index_3 2)
          (`PrimitiveComponent.SetMaterial` _array_element_3 0 "/Engine/VREditor/BasicMeshes/MI_Cube_03.MI_Cube_03")
          (else
            (`PrimitiveComponent.SetMaterial` _array_element_3 0 "/Engine/BasicShapes/BasicShapeMaterial.BasicShapeMaterial")))))
    (:`NewEnumerator3`
      (for (_array_element_4 _array_index_4) _array
        (if (== _array_index_4 3)
          (`PrimitiveComponent.SetMaterial` _array_element_4 0 "/Engine/VREditor/BasicMeshes/MI_Cube_03.MI_Cube_03")
          (else
            (`PrimitiveComponent.SetMaterial` _array_element_4 0 "/Engine/BasicShapes/BasicShapeMaterial.BasicShapeMaterial")))))))

(fn `Current Cog State`
  (bind _cogstate (`self.cogState`))
  (if (== _cogstate 0)
    (set `self.cogState` "NewEnumerator3")
    (else
      (set `self.cogState` (cast `/Game/Patryk_Klich/CogEnum` (- _cogstate 1))))))

(fn `Current Cog State ClockWise`
  (bind _cogstate (`self.cogState`))
  (if (== _cogstate 3)
    (set `self.cogState` "NewEnumerator0")
    (else
      (set `self.cogState` (cast `/Game/Patryk_Klich/CogEnum` (+ _cogstate 1))))))

(fn `UserConstructionScript`
  (bind _returnvalue (`self.K2_GetActorRotation`))
  (`|ExecutionSequence`
    (:`then_0`
      (`self.adjustRotation`))
    (:`then_1`
      (set `self.Gear Rotation` _returnvalue)
      (set `self.GearEnd Rotation` _returnvalue))))