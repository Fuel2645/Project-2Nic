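; Puzzle crank the player turns from inside its trigger box to drive cog trains linked to statues.
; Interact attaches the player with movement disabled while a timeline rotates the crank by Angle, then releases them.
; Two cog arrays start turning in order, each halting at the first missing cog.
; The right statue spins when its chain completes; the left's last-index check (Length - -1) never matches, so it never spins.
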(event `CogRotation`
  (bind _cogarray2 (`self.CogArray2`))
  (bind _cogarray (`self.CogArray`))
  (`|ExecutionSequence`
    (:`then_0`
      (for (_array_element _array_index) _cogarray
        (if (not (`/Game/Patryk_Klich/puzzles/BP_CogPuzzle.Missing` _array_element))
          (`/Game/Patryk_Klich/puzzles/BP_CogPuzzle.TurningStart` _array_element)
          (if (== _array_index (- (`KismetArrayLibrary.Array_Length` _cogarray) 1))
            (`/Game/Patryk_Klich/puzzles/BP_CogStatue.Spin` (`self.StatueRefRight`)))
          (else
            (break)))))
    (:`then_1`
      (if (`KismetArrayLibrary.Array_IsValidIndex` _cogarray2)
        (for (_array_element_2 _array_index_2) _cogarray2
          (if (not (`/Game/Patryk_Klich/puzzles/BP_CogPuzzle.Missing` _array_element_2))
            (`/Game/Patryk_Klich/puzzles/BP_CogPuzzle.TurningStart` _array_element_2)
            (if (== _array_index_2 (- (`KismetArrayLibrary.Array_Length` _cogarray2) -1))
              (`/Game/Patryk_Klich/puzzles/BP_CogStatue.Spin` (`self.StatueRefLeft`)))
            (else
              (break))))))))

(event `/Game/Luke_Dev/BPI_Interact.Interact`
  (params (Instigator :type "/Game/MainBuild/MainCharacter/BP_MainCharceter_Correct Object Reference"))
  (bind _returnvalue (`GameplayStatics.GetPlayerCharacter` 0))
  (if (`self.CorrectPlace`)
    (`CharacterMovementComponent.DisableMovement` (`Character.CharacterMovement` _returnvalue))
    (`self.K2_AttachToComponent` _returnvalue (`self.Cube`) "None" "KeepWorld" "KeepWorld" "KeepWorld" true)
    (`self.Rotate`)
    (`self.CogRotation`)))

(event `Rotate`
  (bind (_crank_rotation_roll _crank_rotation_pitch _crank_rotation_yaw) (`KismetMathLibrary.BreakRotator` (`self.Crank Rotation`)))
  (bind (_crank_rotation_roll_2 _crank_rotation_pitch_2 _crank_rotation_yaw_2) (`KismetMathLibrary.BreakRotator` (`self.Crank Rotation`)))
  (set `self.Crank End Rotation` (`KismetMathLibrary.MakeRotator` _crank_rotation_roll _crank_rotation_pitch (+ _crank_rotation_yaw (`self.Angle`))))
  (bind (_direction _newtrack_0) (`Timeline|Timeline` :!via `PlayFromStart`)
    (:`Update`
      (`SceneComponent.K2_SetRelativeRotation` (`self.Cylinder`) (`KismetMathLibrary.RLerp` (`self.Crank Rotation`) (`self.Crank End Rotation`) _newtrack_0) false false))
    (:`Finished`
      (`self.Stop Rotating`)
      (set `self.Crank Rotation` (`KismetMathLibrary.MakeRotator` _crank_rotation_roll_2 _crank_rotation_pitch_2 (+ _crank_rotation_yaw_2 (`self.Angle`)))))))

(event `self.Box.OnComponentBeginOverlap`
  (params (OverlappedComponent :type "PrimitiveComponent Object Reference") (OtherActor :type "Actor Object Reference") (OtherComp :type "PrimitiveComponent Object Reference") (OtherBodyIndex :type Integer) (bFromSweep :type Boolean) (SweepResult :type "HitResult Structure (by ref)"))
  (if (== OtherComp (`Character.CapsuleComponent` (`GameplayStatics.GetPlayerCharacter` 0)))
    (set `self.CorrectPlace` true)))

(event `self.Box.OnComponentEndOverlap`
  (params (OverlappedComponent :type "PrimitiveComponent Object Reference") (OtherActor :type "Actor Object Reference") (OtherComp :type "PrimitiveComponent Object Reference") (OtherBodyIndex :type Integer))
  (if (== OtherComp (`Character.CapsuleComponent` (`GameplayStatics.GetPlayerCharacter` 0)))
    (set `self.CorrectPlace` false)))

(event `Stop Rotating`
  (bind _returnvalue (`GameplayStatics.GetPlayerCharacter` 0))
  (`CharacterMovementComponent.SetMovementMode` (`Character.CharacterMovement` _returnvalue) "MOVE_Walking" 0)
  (`self.K2_DetachFromActor` _returnvalue "KeepWorld" "KeepWorld" "KeepWorld"))

(fn `UserConstructionScript`)