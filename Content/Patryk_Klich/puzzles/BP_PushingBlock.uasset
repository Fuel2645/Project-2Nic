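; A puzzle block that the player character pushes a fixed travel distance by walking into it.
; On hit, it gets a push direction from the hit normal, then line-traces to confirm the player faces it and box-traces that the path is clear.
; A timeline slides the block while the player is attached with movement disabled, then restores walking and detaches.
; BeginPlay also spawns an actor at the block's Destination offset.
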(event `self.ReceiveBeginPlay`
  (`|ExecutionSequence`
    (:`then_0`
      (`|SpawnActorFromClass` "/Game/Patryk_Klich/puzzles/BP_PressurePlate.BP_PressurePlate_C" (`KismetMathLibrary.MakeTransform` (+ (`self.K2_GetActorLocation`) (`self.Destination`))) "Undefined" "MultiplyWithRoot" null null))))

(event `self.ReceiveHit`
  (params (MyComp :type "PrimitiveComponent Object Reference") (Other :type "Actor Object Reference") (OtherComp :type "PrimitiveComponent Object Reference") (bSelfMoved :type Boolean) (HitLocation :type "Vector Structure") (HitNormal :type "Vector Structure") (NormalImpulse :type "Vector Structure") (Hit :type "HitResult Structure (by ref)"))
  (bind _returnvalue (`GameplayStatics.GetPlayerCharacter` 0))
  (bind (_returnvalue_2 _returnvalue2) (`self.GettingPushDirection` Other HitNormal))
  (if (== Other (`GameplayStatics.GetPlayerCharacter` 0))
    (if _returnvalue2
      (set `self.PushableDirection` _returnvalue_2)
      (bind _canpush (`self.CanPush`))
      (if _canpush
        (`CharacterMovementComponent.DisableMovement` (`Character.CharacterMovement` _returnvalue))
        (`self.K2_AttachToActor` _returnvalue self "None" "KeepWorld" "KeepWorld" "KeepWorld" true)
        (`self.Push`)))))

(event `Push`
  (set `self.CurrentLocation` (`self.K2_GetActorLocation`))
  (bind (_direction _position) (`Timeline|MoveBlock` :!via `PlayFromStart`)
    (:`Update`
      (`self.K2_SetActorRelativeLocation` (+ (* _position (`self.PushableDirection`) (`self.TravelDistance`)) (`self.CurrentLocation`))))
    (:`Finished`
      (`self.StopPushing`))))

(event `StopPushing`
  (bind _returnvalue (`GameplayStatics.GetPlayerCharacter` 0))
  (`CharacterMovementComponent.SetMovementMode` (`Character.CharacterMovement` _returnvalue) "MOVE_Walking" 0)
  (`self.K2_DetachFromActor` _returnvalue "KeepWorld" "KeepWorld" "KeepWorld"))

(fn `CanPush`
  (returns (CanPush :type Boolean))
  (bind _returnvalue (`GameplayStatics.GetPlayerCharacter` 0))
  (bind _returnvalue_2 (`self.K2_GetActorLocation`))
  (bind _cube (`self.Cube`))
  (bind _returnvalue_3 (`self.K2_GetActorLocation` _returnvalue))
  (bind (_returnvalue_origin _returnvalue_boxextent) (`KismetMathLibrary.BreakBoxSphereBounds` (`StaticMesh.GetBounds` (`StaticMeshComponent.StaticMesh` _cube))))
  (bind (_outhit _returnvalue_4) (`KismetSystemLibrary.LineTraceSingle` _returnvalue_3 (+ _returnvalue_3 (* (`self.GetActorForwardVector` _returnvalue) 100.0)) "TraceTypeQuery1" false (`|MakeArray` _returnvalue :!type "Actor Object Reference") "None" false))
  (if _returnvalue_4
    (if (== (`.HitActor` (`GameplayStatics.BreakHitResult` _outhit)) self)
      (bind (_outhit_2 _returnvalue_5) (`KismetSystemLibrary.BoxTraceSingle` :`Start` (+ _returnvalue_2 (0.0 0.0 10.0)) :`End` (+ _returnvalue_2 (* (`self.PushableDirection`) (`self.TravelDistance`)) (0.0 0.0 10.0)) :`HalfSize` (* _returnvalue_boxextent (`SceneComponent.RelativeScale3D` _cube) (0.9 0.9 0.9)) :`TraceChannel` "TraceTypeQuery1" :`DrawDebugType` "ForDuration"))
      (return (not _returnvalue_5))
      (else
        (return false)))))

(fn `UserConstructionScript`)