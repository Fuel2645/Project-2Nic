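; BP_CogStatue is a puzzle statue that rotates in steps about its yaw axis when Spin is triggered.
; Spin computes an end rotation by adding Angle to the stored yaw, then a Timeline lerps the Cube's relative rotation toward it.
; When the Timeline finishes, the stored rotation advances by Angle, so each completed spin builds on the last.
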(event `Spin`
  (bind (_statue_rotation_roll _statue_rotation_pitch _statue_rotation_yaw) (`KismetMathLibrary.BreakRotator` (`self.Statue Rotation`)))
  (bind (_statue_rotation_roll_2 _statue_rotation_pitch_2 _statue_rotation_yaw_2) (`KismetMathLibrary.BreakRotator` (`self.Statue Rotation`)))
  (set `self.Statue End Rotation` (`KismetMathLibrary.MakeRotator` _statue_rotation_roll_2 _statue_rotation_pitch_2 (+ _statue_rotation_yaw_2 (`self.Angle`))))
  (bind (_direction _newtrack_0) (`Timeline|Timeline` :!via `PlayFromStart`)
    (:`Update`
      (`SceneComponent.K2_SetRelativeRotation` (`self.Cube`) (`KismetMathLibrary.RLerp` (`self.Statue Rotation`) (`self.Statue End Rotation`) _newtrack_0) false false))
    (:`Finished`
      (set `self.Statue Rotation` (`KismetMathLibrary.MakeRotator` _statue_rotation_roll _statue_rotation_pitch (+ _statue_rotation_yaw (`self.Angle`)))))))

(fn `UserConstructionScript`)