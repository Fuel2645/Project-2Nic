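; Breakable prop actor covering urns, crates, fences, bushes, bones and caskets, with a geometry collection body set from Model at construction.
; BeginPlay enables overlap collision on the component matching its item-type enum.
; Overlaps passing a hit check destroy the actor after three seconds.
; Middle fence and crate test for projectiles (the crate's class input is unconnected); others call SwordHitCheck, whose player-component comparison is unused.
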(event `self.ReceiveBeginPlay`
  (switch `/Game/Patryk_Klich/BreakableItemEnum` (`self.Enum`)
    (:`NewEnumerator0`
      (`PrimitiveComponent.SetCollisionProfileName` (`self.UrnBox`) "OverlapAllDynamic" true))
    (:`NewEnumerator1`
      (`PrimitiveComponent.SetCollisionProfileName` (`self.CrateBox`) "OverlapAllDynamic" true))
    (:`NewEnumerator2`
      (`PrimitiveComponent.SetCollisionProfileName` (`self.BonePile`) "OverlapAllDynamic" true))
    (:`NewEnumerator3`
      (`PrimitiveComponent.SetCollisionProfileName` (`self.BrokenFence`) "OverlapAllDynamic" true))
    (:`NewEnumerator4`
      (`PrimitiveComponent.SetCollisionProfileName` (`self.SlantedFence`) "OverlapAllDynamic" true))
    (:`NewEnumerator5`
      (`PrimitiveComponent.SetCollisionProfileName` (`self.MiddleFence`) "OverlapAllDynamic" true))
    (:`NewEnumerator6`
      (`PrimitiveComponent.SetCollisionProfileName` (`self.RoseBush`) "OverlapAllDynamic" true))
    (:`NewEnumerator7`
      (`PrimitiveComponent.SetCollisionProfileName` (`self.SkullPile`) "OverlapAllDynamic" true))
    (:`NewEnumerator8`
      (`PrimitiveComponent.SetCollisionProfileName` (`self.Skull`) "OverlapAllDynamic" true))
    (:`NewEnumerator9`
      (`PrimitiveComponent.SetCollisionProfileName` (`self.Bush`) "OverlapAllDynamic" true))
    (:`NewEnumerator10`
      (`PrimitiveComponent.SetCollisionProfileName` (`self.OpenCasket`) "OverlapAllDynamic" true))
    (:`NewEnumerator11`
      (`PrimitiveComponent.SetCollisionProfileName` (`self.ClosedCasket`) "OverlapAllDynamic" true))))

(event `self.MiddleFence.OnComponentBeginOverlap`
  (params (OverlappedComponent :type "PrimitiveComponent Object Reference") (OtherActor :type "Actor Object Reference") (OtherComp :type "PrimitiveComponent Object Reference") (OtherBodyIndex :type Integer) (bFromSweep :type Boolean) (SweepResult :type "HitResult Structure (by ref)"))
  (if (`KismetMathLibrary.ClassIsChildOf` (`GameplayStatics.GetObjectClass` OtherActor) "/Game/Design_Luke/ProjectileChildren/BP_ParentProjectile.BP_ParentProjectile_C")
    (`KismetSystemLibrary.Delay` 3.0 :!label _label)
    (`self.K2_DestroyActor`)))

(event `self.SlantedFence.OnComponentBeginOverlap`
  (params (OverlappedComponent :type "PrimitiveComponent Object Reference") (OtherActor :type "Actor Object Reference") (OtherComp :type "PrimitiveComponent Object Reference") (OtherBodyIndex :type Integer) (bFromSweep :type Boolean) (SweepResult :type "HitResult Structure (by ref)"))
  (if (`self.SwordHitCheck` OtherComp)
    (goto _label)))

(event `self.BrokenFence.OnComponentBeginOverlap`
  (params (OverlappedComponent :type "PrimitiveComponent Object Reference") (OtherActor :type "Actor Object Reference") (OtherComp :type "PrimitiveComponent Object Reference") (OtherBodyIndex :type Integer) (bFromSweep :type Boolean) (SweepResult :type "HitResult Structure (by ref)"))
  (if (`self.SwordHitCheck` OtherComp)
    (goto _label)))

(event `self.BonePile.OnComponentBeginOverlap`
  (params (OverlappedComponent :type "PrimitiveComponent Object Reference") (OtherActor :type "Actor Object Reference") (OtherComp :type "PrimitiveComponent Object Reference") (OtherBodyIndex :type Integer) (bFromSweep :type Boolean) (SweepResult :type "HitResult Structure (by ref)"))
  (if (`self.SwordHitCheck` OtherComp)
    (goto _label)))

(event `self.CrateBox.OnComponentBeginOverlap`
  (params (OverlappedComponent :type "PrimitiveComponent Object Reference") (OtherActor :type "Actor Object Reference") (OtherComp :type "PrimitiveComponent Object Reference") (OtherBodyIndex :type Integer) (bFromSweep :type Boolean) (SweepResult :type "HitResult Structure (by ref)"))
  (if (`KismetMathLibrary.ClassIsChildOf` (`GameplayStatics.GetObjectClass` null) "/Game/Design_Luke/ProjectileChildren/BP_ParentProjectile.BP_ParentProjectile_C")
    (goto _label)))

(event `self.UrnBox.OnComponentBeginOverlap`
  (params (OverlappedComponent :type "PrimitiveComponent Object Reference") (OtherActor :type "Actor Object Reference") (OtherComp :type "PrimitiveComponent Object Reference") (OtherBodyIndex :type Integer) (bFromSweep :type Boolean) (SweepResult :type "HitResult Structure (by ref)"))
  (if (`self.SwordHitCheck` OtherComp)
    (goto _label)))

(event `self.ClosedCasket.OnComponentBeginOverlap`
  (params (OverlappedComponent :type "PrimitiveComponent Object Reference") (OtherActor :type "Actor Object Reference") (OtherComp :type "PrimitiveComponent Object Reference") (OtherBodyIndex :type Integer) (bFromSweep :type Boolean) (SweepResult :type "HitResult Structure (by ref)"))
  (if (`self.SwordHitCheck` OtherComp)
    (goto _label)))

(event `self.OpenCasket.OnComponentBeginOverlap`
  (params (OverlappedComponent :type "PrimitiveComponent Object Reference") (OtherActor :type "Actor Object Reference") (OtherComp :type "PrimitiveComponent Object Reference") (OtherBodyIndex :type Integer) (bFromSweep :type Boolean) (SweepResult :type "HitResult Structure (by ref)"))
  (if (`self.SwordHitCheck` OtherComp)
    (goto _label)))

(event `self.RoseBush.OnComponentBeginOverlap`
  (params (OverlappedComponent :type "PrimitiveComponent Object Reference") (OtherActor :type "Actor Object Reference") (OtherComp :type "PrimitiveComponent Object Reference") (OtherBodyIndex :type Integer) (bFromSweep :type Boolean) (SweepResult :type "HitResult Structure (by ref)"))
  (if (`self.SwordHitCheck` OtherComp)
    (goto _label)))

(event `self.Bush.OnComponentBeginOverlap`
  (params (OverlappedComponent :type "PrimitiveComponent Object Reference") (OtherActor :type "Actor Object Reference") (OtherComp :type "PrimitiveComponent Object Reference") (OtherBodyIndex :type Integer) (bFromSweep :type Boolean) (SweepResult :type "HitResult Structure (by ref)"))
  (if (`self.SwordHitCheck` OtherComp)
    (goto _label)))

(event `self.Skull.OnComponentBeginOverlap`
  (params (OverlappedComponent :type "PrimitiveComponent Object Reference") (OtherActor :type "Actor Object Reference") (OtherComp :type "PrimitiveComponent Object Reference") (OtherBodyIndex :type Integer) (bFromSweep :type Boolean) (SweepResult :type "HitResult Structure (by ref)"))
  (if (`self.SwordHitCheck` OtherComp)
    (goto _label)))

(event `self.SkullPile.OnComponentBeginOverlap`
  (params (OverlappedComponent :type "PrimitiveComponent Object Reference") (OtherActor :type "Actor Object Reference") (OtherComp :type "PrimitiveComponent Object Reference") (OtherBodyIndex :type Integer) (bFromSweep :type Boolean) (SweepResult :type "HitResult Structure (by ref)"))
  (if (`self.SwordHitCheck` OtherComp)
    (goto _label)))

(fn `UserConstructionScript`
  (`GeometryCollectionComponent.SetRestCollection` (`self.body`) (`self.model`)))