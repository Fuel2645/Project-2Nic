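; Player character Blueprint with a dash that leads into sprinting while the dash input is held.
; A timeline drives horizontal velocity along the forward vector and calls StartSprinting on each update, raising walk speed.
; Releasing the input calls StopSprinting to lower it.
; Stamina drain and regen events loop through delayed self-calls with debug prints, but their calls in the sprint functions are unwired, so stamina never changes.
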(event `EnhancedInput|/Game/Daniel_A/Input/Actions/IA_Dash`
  (params (ActionValue :type Boolean) (ElapsedSeconds :type "Float (double-precision)") (TriggeredSeconds :type "Float (double-precision)") (InputAction :type "InputAction Object Reference" :default "/Game/Daniel_A/Input/Actions/IA_Dash.IA_Dash"))
  (bind (_velocity_x _velocity_y _velocity_z) (`KismetMathLibrary.BreakVector` (`MovementComponent.Velocity` (`self.CharacterMovement`))))
  (:`Started`
    (bind (_direction _distance) (`Timeline|Timeline` :!via `PlayFromStart`)
      (:`Update`
        (bind (_returnvalue_x _returnvalue_y) (`KismetMathLibrary.BreakVector` (* (`self.GetActorForwardVector`) (* _distance (`self.Dash Distance`)))))
        (set `MovementComponent.Velocity` (`KismetMathLibrary.MakeVector` _returnvalue_x _returnvalue_y _velocity_z) (`self.CharacterMovement`))
        (`self.StartSprinting`))))
  (:`Completed`
    (`self.StopSprinting`)))

(event `StamDrain`
  (bind _output_get (set `self.Stamina` (`KismetMathLibrary.Clamp` (- (`self.Stamina`) 1) 0 (`self.MaxStamina`))))
  (if (== _output_get 0)
    (`self.StopSprinting`)
    (elif (`self.isSprinting`)
      (`KismetSystemLibrary.Delay` 0.1)
      (`self.StamDrain`)
      (`KismetSystemLibrary.PrintString` (`KismetStringLibrary.Conv_IntToString` (`self.Stamina`))))))

(event `StaminaRegen`
  (bind _output_get (set `self.Stamina` (`KismetMathLibrary.Clamp` (+ (`self.Stamina`) 5) 0 (`self.MaxStamina`))))
  (if (== _output_get (`self.MaxStamina`))
    _
    (elif (not (`self.isSprinting`))
      (`KismetSystemLibrary.Delay` 0.5)
      (`self.StaminaRegen`)
      (`KismetSystemLibrary.PrintString` (`KismetStringLibrary.Conv_IntToString` (`self.Stamina`))))))

(fn `StartSprinting`
  (set `CharacterMovementComponent.MaxWalkSpeed` 600.0 (`self.CharacterMovement`))
  (set `self.isSprinting` true))

(fn `StopSprinting`
  (set `CharacterMovementComponent.MaxWalkSpeed` 300.0 (`self.CharacterMovement`))
  (set `self.isSprinting` false))

(fn `UserConstructionScript`
  (`parent.UserConstructionScript`))