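; Test character Blueprint for stamina-based dash and sprint movement on a single input; no camera logic appears here.
; Pressing dash with enough stamina runs a timeline that drives horizontal velocity along the last input vector, granting invulnerability.
; Holding the input starts sprinting; a dash costs stamina only if the input is released when its post-dash cooldown ends.
; Delay-looped custom events drain or regenerate stamina, calling UpdateStamina and printing debug values.
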(event `EnhancedInput|/Game/Daniel_A/Input/Actions/IA_Dash`
  (params (ActionValue :type Boolean) (ElapsedSeconds :type "Float (double-precision)") (TriggeredSeconds :type "Float (double-precision)") (InputAction :type "InputAction Object Reference" :default "/Game/Daniel_A/Input/Actions/IA_Dash.IA_Dash"))
  (bind (_velocity_x _velocity_y _velocity_z) (`KismetMathLibrary.BreakVector` (`MovementComponent.Velocity` (`self.CharacterMovement`))))
  ;[1 0.9044 0] Dash/Sprint
  (:`Triggered`
    (`self.StartSprinting`))
  (:`Started`
    (if (`self.Just Dashed`)
      _
      (elif (> (`self.Stamina`) 100.0)
        (set `self.isDashing` true)
        (set `self.Just Dashed` true)
        (set `self.Invulnerable` true)
        (bind (_direction _distance) (`Timeline|Timeline_0` :!via `PlayFromStart`)
          (:`Update`
            (bind (_returnvalue_x _returnvalue_y) (`KismetMathLibrary.BreakVector` (* (`self.GetLastMovementInputVector`) (* _distance (`self.Dash Distance`)))))
            (set `MovementComponent.Velocity` (`KismetMathLibrary.MakeVector` _returnvalue_x _returnvalue_y _velocity_z) (`self.CharacterMovement`))
            (if (`|GetInputActionValue`)
              (`self.StartSprinting`)))
          (:`Finished`
            (set `self.Invulnerable` false)
            (if (`self.Just Dashed`)
              (`KismetSystemLibrary.Delay` 1.0)
              (set `self.Just Dashed` false)
              (set `self.isDashing` false)
              (if (not (`|GetInputActionValue`))
                (set `self.Stamina` (`KismetMathLibrary.Clamp` (- (`self.Stamina`) 100) 0 (`self.Max Stamina`)))
                (`KismetSystemLibrary.PrintString` (`KismetStringLibrary.Conv_IntToString` (`self.Stamina`))))))))))
  (:`Completed`
    (`self.StopSprinting`)))

(event `CustomEvent`
  (bind _stamina (`self.Stamina`))
  ;[1 0.9044 0] Stamina Drain/Regen
  (bind _output_get (set `self.Stamina` (`KismetMathLibrary.Clamp` (- (`self.Stamina`) 1) 0 (`self.Max Stamina`))))
  (if (== _output_get 0)
    (`self.StopSprinting`)
    (elif (`self.isSprinting`)
      (`KismetSystemLibrary.Delay` 0.1)
      (`self.StaminaDrain`)
      (`KismetSystemLibrary.PrintString` (`KismetStringLibrary.Conv_IntToString` _stamina) true true (struct :`G` 0.66 :`B` 1.0 :`A` 1.0) 0.1)
      (`self.Update Stamina` (`KismetMathLibrary.Conv_IntToDouble` _stamina)))))

(event `CustomEvent_1`
  (bind _stamina (`self.Stamina`))
  ;[1 0.9044 0] Stamina Drain/Regen
  (bind _output_get (set `self.Stamina` (`KismetMathLibrary.Clamp` (+ (`self.Stamina`) 2) 0 (`self.Max Stamina`))))
  (if (not (== _output_get (`self.Max Stamina`)))
    (`KismetSystemLibrary.Delay` 0.1)
    (`self.StaminaRegen`)
    (`KismetSystemLibrary.PrintString` (`KismetStringLibrary.Conv_IntToString` _stamina) true true (struct :`G` 0.66 :`B` 1.0 :`A` 1.0) 0.1)
    (`self.Update Stamina` (`KismetMathLibrary.Conv_IntToDouble` _stamina))))

(fn `UserConstructionScript`
  (`parent.UserConstructionScript`))